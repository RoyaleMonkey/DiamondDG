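; BP_DecalLore is a decal Blueprint, filed under lore decals, whose color and texture are configurable through variables.
; On BeginPlay it creates a dynamic material instance from the decal's material, assigns it back to the decal, and pushes the Color and TextureDecal values into the matching parameters.
; The construction script is empty, so these values are applied only at runtime.
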(event EventBeginPlay
  (bind _returnvalue (Rendering|Material|CreateDynamicMaterialInstance (Class|DecalComponent|GetDecalMaterial (Variables|Default|GetDecal)) "None" "None" :!class /Script/Engine.KismetMaterialLibrary))
  (bind _output_get (Variables|Default|SetMaterialInstance _returnvalue))
  (Rendering|Components|Decal|SetDecalMaterial (Variables|Default|GetDecal) _output_get)
  (Rendering|Material|SetVectorParameterValue (Variables|Default|GetMaterialInstance) "Color" (Variables|Default|GetColor) :!class /Script/Engine.MaterialInstanceDynamic)
  (Rendering|Material|SetTextureParameterValue (Variables|Default|GetMaterialInstance) "TextureDecal" (Variables|Default|GetTextureDecal)))

(fn ConstructionScript)