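; BreakObjectComponent is an actor component that lets its GlobalCharacter owner destroy objects tagged Breakable.
; Each tick it line-traces a short distance forward from the follow camera on the Visibility channel, ignoring the owner, storing a tagged hit as Target and updating CanBreak.
; UseBreakPower destroys that Target when CanBreak is true.
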(event EventTick
  (params (DeltaSeconds :type Float%20%28single-precision%29))
  (bind _asglobal_character (Utilities|Casting|CastToGlobalCharacter (Components|GetOwner)))
  (bind (_outhit _returnvalue) (Collision|LineTraceByChannel (Transformation|GetWorldLocation (Variables|/Script/DesignGate.DesignGateCharacter|GetFollowCamera _asglobal_character)) (+ (Transformation|GetWorldLocation (Variables|/Script/DesignGate.DesignGateCharacter|GetFollowCamera _asglobal_character)) (* (Math|Vector|GetForwardVector (Variables|/Script/DesignGate.DesignGateCharacter|GetFollowCamera _asglobal_character)) 5e+02)) "TraceTypeQuery1" false (Utilities|Array|MakeArray _asglobal_character) "None"))
  (if _returnvalue
    (if (Actor|ActorHasTag (.HitActor (Collision|BreakHitResult _outhit)) "Breakable")
      (Variables|Default|SetTarget (.HitActor (Collision|BreakHitResult _outhit)))
      (Variables|Default|SetCanBreak true)
      (else
        (Variables|Default|SetCanBreak false :!label _label)))
    (else
      (goto _label))))

(fn UseBreakPower
  (if (Variables|Default|GetCanBreak)
    (Actor|DestroyActor (Variables|Default|GetTarget))))