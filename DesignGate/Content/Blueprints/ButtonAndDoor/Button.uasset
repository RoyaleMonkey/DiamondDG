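; Pressure button actor that sinks by PressureDepth while other actors overlap its Box component.
; Overlap events track those actors in ObjectsOnButton, setting IsActivated on entry and clearing it only when the last one leaves.
; While active, Tick repeatedly sweeps the button to the pressed position cached at BeginPlay, and release immediately sweeps it back to its default position.
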(event OnComponentBeginOverlap(Box)
  (params (OverlappedComponent :type Primitive%20Component%20Object%20Reference) (OtherActor :type Actor%20Object%20Reference) (OtherComp :type Primitive%20Component%20Object%20Reference) (OtherBodyIndex :type Integer) (bFromSweep :type Boolean) (SweepResult :type Hit%20Result%20Structure%20%28by%20ref%29))
  (if (!= OtherActor self)
    (Utilities|Array|AddUnique (Variables|Default|GetObjectsOnButton) OtherActor)
    (if (not (Variables|Default|GetIsActivated))
      (Variables|Default|SetIsActivated true))))

(event OnComponentEndOverlap(Box)
  (params (OverlappedComponent :type Primitive%20Component%20Object%20Reference) (OtherActor :type Actor%20Object%20Reference) (OtherComp :type Primitive%20Component%20Object%20Reference) (OtherBodyIndex :type Integer))
  (if (!= OtherActor self)
    (Utilities|Array|RemoveItem (Variables|Default|GetObjectsOnButton) OtherActor)
    (if (== (Utilities|Array|Length (Variables|Default|GetObjectsOnButton)) 0)
      (Variables|Default|SetIsActivated false)
      (Transformation|SetActorLocation (Variables|Default|GetDefaultPosition) true false))))

(event EventTick
  (params (DeltaSeconds :type Float%20%28single-precision%29))
  (if (Variables|Default|GetIsActivated)
    (Transformation|SetActorLocation (Variables|Default|GetPressedPosition) true false)))

(event EventBeginPlay
  (bind _returnvalue (Transformation|GetActorLocation))
  (Variables|Default|SetDefaultPosition (Transformation|GetActorLocation))
  (Variables|Default|SetPressedPosition (Math|Vector|MakeVector (.x _returnvalue) (.y _returnvalue) (- (.z _returnvalue) (Variables|Default|GetPressureDepth)))))

(fn ConstructionScript)