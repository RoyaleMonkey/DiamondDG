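; Puzzle door that opens by toggle when interactable, or otherwise while all linked buttons, levers and stacked telekinetic objects are satisfied.
; Tick lerps it over a set duration in one of six swing or slide modes, with slide distance defaulting to mesh size when negative.
; Stack checks use upward line traces and snap objects into place.
; If the condition flips mid-motion, elapsed time is mirrored to reverse smoothly.
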(event EventBeginPlay
  (bind _staticmesh (Variables|Default|GetStaticMesh))
  (bind _returnvalue (Transformation|GetWorldScale _staticmesh))
  (bind (_min _max) (Components|StaticMesh|GetLocalBounds _staticmesh))
  (Variables|Default|SetMeshSize (+ (* (* _min _returnvalue) -1.0) (* _max _returnvalue))))

(event EventTick
  (params (DeltaSeconds :type Float%20%28single-precision%29))
  (if (Variables|Default|GetInteractable)
    (if (Variables|Default|GetToggleOpen)
      (if (not (Variables|Default|GetIsOpen)) :!label _label
        (Variables|Default|SetIsClose false)
        (if (Variables|Default|GetIsMoving)
          _
          (else
            (Variables|Default|SetActualOpenCloseDuration 0.0)
            (Variables|Default|SetIsMoving true)))
        (Variables|Default|SetActualOpenCloseDuration (+ (Variables|Default|GetActualOpenCloseDuration) DeltaSeconds))
        (CallFunction|Open)
        (if (>= (Variables|Default|GetActualOpenCloseDuration) (Variables|Default|GetOpenCloseDuration))
          (Variables|Default|SetIsOpen true)
          (Variables|Default|SetIsMoving false :!label _label_2)))
      (else
        (if (not (Variables|Default|GetIsClose)) :!label _label_3
          (Variables|Default|SetIsOpen false)
          (if (Variables|Default|GetIsMoving)
            _
            (else
              (Variables|Default|SetActualOpenCloseDuration 0.0)
              (Variables|Default|SetIsMoving true)))
          (Variables|Default|SetActualOpenCloseDuration (+ (Variables|Default|GetActualOpenCloseDuration) DeltaSeconds))
          (CallFunction|Close)
          (if (>= (Variables|Default|GetActualOpenCloseDuration) (Variables|Default|GetOpenCloseDuration))
            (Variables|Default|SetIsClose true)
            (goto _label_2)))))
    (else
      (bind _canopen (CallFunction|CheckButtonsandLevers))
      (if _canopen
        (goto _label)
        (else
          (goto _label_3))))))

(fn ConstructionScript)

(fn CheckButtonsandLevers
  (Variables|Check|SetAllTelekineticObjectsStacked true)
  (Variables|Check|SetAllButtons true)
  (Variables|Check|SetAllLevers true)
  (bind _array_element (Utilities|Array|ForEachLoopwithBreak (Variables|Default|GetButtons) :!label _label)
    (:LoopBody
      (Utilities|IsValid _array_element
        (:Is%20Valid
          (if (not (Variables|/Game/Blueprints/ButtonAndDoor/Button.Button_C|GetIsActivated _array_element))
            (Variables|Check|SetAllButtons false)
            (goto _label Break)))))
    (:Completed
      (bind _array_element_2 (Utilities|Array|ForEachLoopwithBreak (Variables|Default|GetLevers) :!label _label_2)
        (:LoopBody
          (Utilities|IsValid _array_element_2
            (:Is%20Valid
              (if (not (Variables|/Game/Blueprints/ButtonAndDoor/Lever.Lever_C|GetIsActivated _array_element_2))
                (Variables|Check|SetAllLevers false)
                (goto _label_2 Break)))))
        (:Completed
          (for _array_element_3 (Variables|Default|GetStackedTelekineticObjects)
            (for (_array_element_4 _array_index) (Utilities|Struct|BreakStackedTelekineticObjects _array_element_3)
              (Utilities|IsValid _array_element_4
                (:Is%20Valid
                  (if (< _array_index (- (Utilities|Array|Length (Utilities|Struct|BreakStackedTelekineticObjects _array_element_3)) 1))
                    (bind (_outhit _returnvalue) (Collision|LineTraceByChannel (Transformation|GetActorLocation _array_element_4) (+ (Transformation|GetActorLocation _array_element_4) (* (Transformation|GetActorUpVector _array_element_4) (.z (* (.Max (Components|StaticMesh|GetLocalBounds (Variables|/Game/Blueprints/Telekinesis/TelekineticObjectBP.TelekineticObjectBP_C|GetObject _array_element_4))) (Transformation|GetWorldScale (Variables|/Game/Blueprints/Telekinesis/TelekineticObjectBP.TelekineticObjectBP_C|GetObject _array_element_4))))) "0,0,20.000000") "TraceTypeQuery2" false (Utilities|Array|MakeArray _array_element_4) "None"))
                    (if _returnvalue
                      (if (== (.HitActor (Collision|BreakHitResult _outhit)) (Utilities|Array|Get(acopy) (Utilities|Struct|BreakStackedTelekineticObjects _array_element_3) (+ _array_index 1)))
                        (CallFunction|SnapObjects _array_element_4 (Utilities|Array|Get(acopy) (Utilities|Struct|BreakStackedTelekineticObjects _array_element_3) (+ _array_index 1)))
                        (else
                          (Variables|Check|SetAllTelekineticObjectsStacked false :!label _label_3)))
                      (else
                        (goto _label_3))))))))
          (if (Math|Boolean|ANDBoolean (Variables|Check|GetAllTelekineticObjectsStacked) (Variables|Check|GetAllButtons) (Variables|Check|GetAllLevers))
            (if (Math|Boolean|ANDBoolean (not (Variables|Default|GetLastCheck)) (> (Variables|Default|GetActualOpenCloseDuration) 0.0) (< (Variables|Default|GetActualOpenCloseDuration) (Variables|Default|GetOpenCloseDuration)))
              (Variables|Default|SetActualOpenCloseDuration (- (Variables|Default|GetOpenCloseDuration) (Variables|Default|GetActualOpenCloseDuration))))
            (Variables|Default|SetLastCheck true)
            (return true)
            (else
              (if (Math|Boolean|ANDBoolean (Variables|Default|GetLastCheck) (> (Variables|Default|GetActualOpenCloseDuration) 0.0) (< (Variables|Default|GetActualOpenCloseDuration) (Variables|Default|GetOpenCloseDuration)))
                (Variables|Default|SetActualOpenCloseDuration (- (Variables|Default|GetOpenCloseDuration) (Variables|Default|GetActualOpenCloseDuration))))
              (Variables|Default|SetLastCheck false)
              (return false))))))))

(fn ClassicRight
  (params (Open :type Boolean))
  (bind _actualopencloseduration (Variables|Default|GetActualOpenCloseDuration))
  (bind _opencloseduration (Variables|Default|GetOpenCloseDuration))
  (bind _right (Variables|Default|GetRight))
  (bind _returnvalue (/ _actualopencloseduration _opencloseduration))
  (if Open
    (Transformation|SetRelativeRotation _right (Math|Rotator|Lerp(Rotator) "0, 0, 0" (Math|Rotator|MakeRotator 0.0 0.0 (Variables|Default|GetRotationAngle)) _returnvalue) false false)
    (else
      (Transformation|SetRelativeRotation _right (Math|Rotator|Lerp(Rotator) (Math|Rotator|MakeRotator 0.0 0.0 (Variables|Default|GetRotationAngle)) "0, 0, 0" _returnvalue) false false))))

(fn ClassicLeft
  (params (Open :type Boolean))
  (bind _left (Variables|Default|GetLeft))
  (bind _actualopencloseduration (Variables|Default|GetActualOpenCloseDuration))
  (bind _opencloseduration (Variables|Default|GetOpenCloseDuration))
  (bind _returnvalue (/ _actualopencloseduration _opencloseduration))
  (if Open
    (Transformation|SetRelativeRotation _left (Math|Rotator|Lerp(Rotator) "0, 0, 0" (Math|Rotator|MakeRotator 0.0 0.0 (* (Variables|Default|GetRotationAngle) -1.0)) _returnvalue) false false)
    (else
      (Transformation|SetRelativeRotation _left (Math|Rotator|Lerp(Rotator) (Math|Rotator|MakeRotator 0.0 0.0 (* (Variables|Default|GetRotationAngle) -1.0)) "0, 0, 0" _returnvalue) false false))))

(fn SlidingLeft
  (params (Open :type Boolean))
  (bind _actualopencloseduration (Variables|Default|GetActualOpenCloseDuration))
  (bind _opencloseduration (Variables|Default|GetOpenCloseDuration))
  (bind _actualopencloseduration_2 (Variables|Default|GetActualOpenCloseDuration))
  (bind _opencloseduration_2 (Variables|Default|GetOpenCloseDuration))
  (bind _right (Variables|Default|GetRight))
  (bind _right_2 (Variables|Default|GetRight))
  (bind _returnvalue (/ _actualopencloseduration _opencloseduration))
  (bind _returnvalue_2 (/ _actualopencloseduration_2 _opencloseduration_2))
  (if (< (Variables|Default|GetSlidingDistance) 0.0)
    (if Open
      (Transformation|SetRelativeLocation _right_2 (Math|Vector|Lerp(Vector) "0, 0, 0" (Math|Vector|MakeVector (/ (.x (Variables|Default|GetMeshSize)) (.x (Transformation|GetActorScale3D))) 0.0 0.0) _returnvalue) false false)
      (else
        (Transformation|SetRelativeLocation _right_2 (Math|Vector|Lerp(Vector) (Math|Vector|MakeVector (/ (.x (Variables|Default|GetMeshSize)) (.x (Transformation|GetActorScale3D))) 0.0 0.0) "0, 0, 0" _returnvalue) false false)))
    (elif Open
      (Transformation|SetRelativeLocation _right (Math|Vector|Lerp(Vector) "0, 0, 0" (Math|Vector|MakeVector (Variables|Default|GetSlidingDistance) 0.0 0.0) _returnvalue_2) false false)
      (else
        (Transformation|SetRelativeLocation _right (Math|Vector|Lerp(Vector) (Math|Vector|MakeVector (Variables|Default|GetSlidingDistance) 0.0 0.0) "0, 0, 0" _returnvalue_2) false false)))))

(fn SlidingRight
  (params (Open :type Boolean))
  (bind _right (Variables|Default|GetRight))
  (bind _actualopencloseduration (Variables|Default|GetActualOpenCloseDuration))
  (bind _opencloseduration (Variables|Default|GetOpenCloseDuration))
  (bind _right_2 (Variables|Default|GetRight))
  (bind _actualopencloseduration_2 (Variables|Default|GetActualOpenCloseDuration))
  (bind _opencloseduration_2 (Variables|Default|GetOpenCloseDuration))
  (bind _returnvalue (/ _actualopencloseduration_2 _opencloseduration_2))
  (bind _returnvalue_2 (/ _actualopencloseduration _opencloseduration))
  (if (< (Variables|Default|GetSlidingDistance) 0.0)
    (if Open
      (Transformation|SetRelativeLocation _right (Math|Vector|Lerp(Vector) "0, 0, 0" (Math|Vector|MakeVector (* (/ (.x (Variables|Default|GetMeshSize)) (.x (Transformation|GetActorScale3D))) -1.0) 0.0 0.0) _returnvalue) false false)
      (else
        (Transformation|SetRelativeLocation _right (Math|Vector|Lerp(Vector) (Math|Vector|MakeVector (* (/ (.x (Variables|Default|GetMeshSize)) (.x (Transformation|GetActorScale3D))) -1.0) 0.0 0.0) "0, 0, 0" _returnvalue) false false)))
    (elif Open
      (Transformation|SetRelativeLocation _right_2 (Math|Vector|Lerp(Vector) "0, 0, 0" (Math|Vector|MakeVector (* (Variables|Default|GetSlidingDistance) -1.0) 0.0 0.0) _returnvalue_2) false false)
      (else
        (Transformation|SetRelativeLocation _right_2 (Math|Vector|Lerp(Vector) (Math|Vector|MakeVector (* (Variables|Default|GetSlidingDistance) -1.0) 0.0 0.0) "0, 0, 0" _returnvalue_2) false false)))))

(fn SlidingTop
  (params (Open :type Boolean))
  (bind _right (Variables|Default|GetRight))
  (bind _actualopencloseduration (Variables|Default|GetActualOpenCloseDuration))
  (bind _opencloseduration (Variables|Default|GetOpenCloseDuration))
  (bind _right_2 (Variables|Default|GetRight))
  (bind _actualopencloseduration_2 (Variables|Default|GetActualOpenCloseDuration))
  (bind _opencloseduration_2 (Variables|Default|GetOpenCloseDuration))
  (bind _returnvalue (/ _actualopencloseduration_2 _opencloseduration_2))
  (bind _returnvalue_2 (/ _actualopencloseduration _opencloseduration))
  (if (< (Variables|Default|GetSlidingDistance) 0.0)
    (if Open
      (Transformation|SetRelativeLocation _right (Math|Vector|Lerp(Vector) "0, 0, 0" (Math|Vector|MakeVector 0.0 0.0 (/ (.z (Variables|Default|GetMeshSize)) (.z (Transformation|GetActorScale3D)))) _returnvalue) false false)
      (else
        (Transformation|SetRelativeLocation _right (Math|Vector|Lerp(Vector) (Math|Vector|MakeVector 0.0 0.0 (/ (.z (Variables|Default|GetMeshSize)) (.z (Transformation|GetActorScale3D)))) "0, 0, 0" _returnvalue) false false)))
    (elif Open
      (Transformation|SetRelativeLocation _right_2 (Math|Vector|Lerp(Vector) "0, 0, 0" (Math|Vector|MakeVector 0.0 0.0 (Variables|Default|GetSlidingDistance)) _returnvalue_2) false false)
      (else
        (Transformation|SetRelativeLocation _right_2 (Math|Vector|Lerp(Vector) (Math|Vector|MakeVector 0.0 0.0 (Variables|Default|GetSlidingDistance)) "0, 0, 0" _returnvalue_2) false false)))))

(fn SlidingBottom
  (params (Open :type Boolean))
  (bind _right (Variables|Default|GetRight))
  (bind _actualopencloseduration (Variables|Default|GetActualOpenCloseDuration))
  (bind _actualopencloseduration_2 (Variables|Default|GetActualOpenCloseDuration))
  (bind _opencloseduration (Variables|Default|GetOpenCloseDuration))
  (bind _right_2 (Variables|Default|GetRight))
  (bind _opencloseduration_2 (Variables|Default|GetOpenCloseDuration))
  (bind _returnvalue (/ _actualopencloseduration _opencloseduration_2))
  (bind _returnvalue_2 (/ _actualopencloseduration_2 _opencloseduration))
  (if (< (Variables|Default|GetSlidingDistance) 0.0)
    (if Open
      (Transformation|SetRelativeLocation _right (Math|Vector|Lerp(Vector) "0, 0, 0" (Math|Vector|MakeVector 0.0 0.0 (* (/ (.z (Variables|Default|GetMeshSize)) (.z (Transformation|GetActorScale3D))) -1.0)) _returnvalue) false false)
      (else
        (Transformation|SetRelativeLocation _right (Math|Vector|Lerp(Vector) (Math|Vector|MakeVector 0.0 0.0 (* (/ (.z (Variables|Default|GetMeshSize)) (.z (Transformation|GetActorScale3D))) -1.0)) "0, 0, 0" _returnvalue) false false)))
    (elif Open
      (Transformation|SetRelativeLocation _right_2 (Math|Vector|Lerp(Vector) "0, 0, 0" (Math|Vector|MakeVector 0.0 0.0 (* (Variables|Default|GetSlidingDistance) -1.0)) _returnvalue_2) false false)
      (else
        (Transformation|SetRelativeLocation _right_2 (Math|Vector|Lerp(Vector) (Math|Vector|MakeVector 0.0 0.0 (* (Variables|Default|GetSlidingDistance) -1.0)) "0, 0, 0" _returnvalue_2) false false)))))

(fn Close
  (switch Utilities|FlowControl|Switch|SwitchonDoorModes (Variables|Default|GetMode)
    (:NewEnumerator1
      (CallFunction|ClassicRight false))
    (:NewEnumerator0
      (CallFunction|ClassicLeft false))
    (:NewEnumerator3
      (CallFunction|SlidingRight false))
    (:NewEnumerator2
      (CallFunction|SlidingLeft false))
    (:NewEnumerator4
      (CallFunction|SlidingTop false))
    (:NewEnumerator5
      (CallFunction|SlidingBottom false))))

(fn Open
  (switch Utilities|FlowControl|Switch|SwitchonDoorModes (Variables|Default|GetMode)
    (:NewEnumerator1
      (CallFunction|ClassicRight true))
    (:NewEnumerator0
      (CallFunction|ClassicLeft true))
    (:NewEnumerator3
      (CallFunction|SlidingRight true))
    (:NewEnumerator2
      (CallFunction|SlidingLeft true))
    (:NewEnumerator4
      (CallFunction|SlidingTop true))
    (:NewEnumerator5
      (CallFunction|SlidingBottom true))))

(fn SnapObjects
  (params (Object1 :type Telekinetic%20Object%20BP%20Object%20Reference) (Object2 :type Telekinetic%20Object%20BP%20Object%20Reference))
  (if (not (Variables|/Game/Blueprints/Telekinesis/TelekineticObjectBP.TelekineticObjectBP_C|GetCanControl Object2))
    (Transformation|SetActorLocation Object2 (+ (Transformation|GetActorLocation Object1) (Math|Vector|MakeVector 0.0 0.0 (- (.z (* (.Max (Components|StaticMesh|GetLocalBounds (Variables|/Game/Blueprints/Telekinesis/TelekineticObjectBP.TelekineticObjectBP_C|GetObject Object1))) (Transformation|GetActorScale3D Object1))) (.z (* (.Min (Components|StaticMesh|GetLocalBounds (Variables|/Game/Blueprints/Telekinesis/TelekineticObjectBP.TelekineticObjectBP_C|GetObject Object2))) (Transformation|GetActorScale3D Object2)))))) false false)))