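; Lever actor with an on/off state, shown by the rotation of a scene component and the material on its ground mesh.
; On BeginPlay it applies the visual state matching its IsActivated flag.
; Activate and Deactivate set the rotation and material for their state and update the flag; the file itself contains no input or trigger logic that toggles it during play.
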(event EventBeginPlay
  (if (Variables|Default|GetIsActivated)
    (CallFunction|Activate)
    (else
      (CallFunction|Deactivate))))

(fn ConstructionScript)

(fn Activate
  (Transformation|SetRelativeRotation (Variables|Default|GetScene) (Variables|Default|GetOnRotation) false false)
  (Rendering|Material|SetMaterial (Variables|Default|Getground) 0 (Variables|Default|GetMaterialOn))
  (Variables|Default|SetIsActivated true))

(fn Deactivate
  (Transformation|SetRelativeRotation (Variables|Default|GetScene) (Variables|Default|GetOffRotation) false false)
  (Rendering|Material|SetMaterial (Variables|Default|Getground) 0 (Variables|Default|GetMaterialOff))
  (Variables|Default|SetIsActivated false))