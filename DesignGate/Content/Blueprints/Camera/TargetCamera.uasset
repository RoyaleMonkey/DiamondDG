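; TargetCamera is a trigger actor that takes over the rotation of the player's follow camera while the player is inside it.
; Begin overlap caches the player as a GlobalCharacter and sets IsUsed, which end overlap clears.
; While IsUsed, Tick sets the FollowCamera's relative rotation with no computed value connected.
; A look-at calculation toward TargetObject exists but is unused, so the camera targeting appears unfinished.
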(event EventTick
  (params (DeltaSeconds :type Float%20%28single-precision%29))
  (if (Variables|Default|GetIsUsed)
    (Transformation|SetRelativeRotation (Variables|/Script/DesignGate.DesignGateCharacter|GetFollowCamera (Variables|Components|GetplayerRef)) (Math|Rotator|MakeRotator 0.0 0.0 0.0) false false)))

(event Collision|EventActorBeginOverlap
  (params (OtherActor :type Actor%20Object%20Reference))
  (if (== OtherActor (Game|GetPlayerCharacter 0))
    (bind _asglobal_character (Utilities|Casting|CastToGlobalCharacter OtherActor))
    (Variables|Components|SetplayerRef _asglobal_character)
    (Variables|Default|SetIsUsed true)))

(event Collision|EventActorEndOverlap
  (params (OtherActor :type Actor%20Object%20Reference))
  (if (== OtherActor (Game|GetPlayerCharacter 0))
    (Variables|Default|SetIsUsed false)))

(fn ConstructionScript)