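; Player character Blueprint combining dash, gliding, pickup/drop/throw and zone-granted red/blue powers, with a toggleable test widget.
; Dash uses a trace-checked MoveComponentTo plus zero-friction inertia; gliding changes gravity, speed and camera boom while tilting the glider.
; A per-tick forward trace finds pickups.
; Option enums select how powers are gained (trigger, buffer, timed key combo), used and lost, spawning a wall or blue sphere.
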(event Custom|AutoGlide
  ;[1 1 1] Glide system
)

(event EventTick
  (params (DeltaSeconds :type Float%20%28single-precision%29))
  (bind _returnvalue (Input|AxisValues|GetMoveRight))
  (bind _glider (Variables|Default|GetGlider))
  (bind _returnvalue_2 (* _returnvalue 15.0))
  (bind _relativerotation (Variables|/Script/Engine.SceneComponent|GetRelativeRotation _glider))
  (bind _returnvalue_3 (Math|Float|Lerp (.roll _relativerotation) _returnvalue_2 0.01))
  ;[1 1 1] Event tick
  ;;[1 1 1] Check Pickup
  (PickupSettings|CheckPickableObjects)
  ;;[1 1 1] Continuous mouvement when gliding
  (if (Variables|GlideSettings|GetisGliding)
    (Pawn|Input|AddMovementInput (* (Transformation|GetActorForwardVector) (Variables|GlideSettings|GetforwardSpeedMultiplier)) 1.0 false)
    (Transformation|SetRelativeRotation _glider (Math|Rotator|MakeRotator _returnvalue_3 (Math|Float|Lerp (.pitch _relativerotation) (* (Input|AxisValues|GetMoveForward) -15.0) 0.01) _returnvalue_3) false false)
    (else
      ;;[1 1 1] Decrement inertia cooldown
      (if (Variables|DashSettings|Private|GetdecreaseInertiaCooldown)
        (Utilities|FlowControl|Delay (Variables|DashSettings|Inertia|GetinertiaDuration))
        (Variables|/Script/Engine.CharacterMovementComponent|SetGroundFriction (Variables|Character|GetCharacterMovement) (Variables|DashSettings|Private|GetgroundFriction))
        (Variables|DashSettings|Private|SetdecreaseInertiaCooldown false)))))

(event EventBeginPlay
  ;[1 1 1] Save normal ground friction for inertia
  (Variables|DashSettings|Private|SetgroundFriction (Variables|/Script/Engine.CharacterMovementComponent|GetGroundFriction (Variables|Character|GetCharacterMovement)))
  (bind _returnvalue (UserInterface|CreateWidget "/Game/Assets/GPAssets/Widget/GlobalTestWidget.GlobalTestWidget_C"))
  (UserInterface|Viewport|AddtoViewport _returnvalue 1)
  (Widget|SetVisibility _returnvalue "Hidden")
  (Variables|Default|SetGlobalTestUI _returnvalue)
  ;[1 1 1] Begin play Power
  (Effects|Components|ParticleSystem|SetEmitterEnable (Variables|Default|GetMainPowerParticle) "Particle Emitter" false)
  (Effects|Components|ParticleSystem|SetEmitterEnable (Variables|Default|GetSecondPowerParticle) "Particle Emitter" false))

(event EventOnLanded
  (params (Hit :type Hit%20Result%20Structure%20%28by%20ref%29))
  (bind _charactermovement (Variables|Character|GetCharacterMovement))
  ;[1 1 1] Glide system
  (Variables|GlideSettings|SetisGliding false)
  (Transformation|AttachComponentToComponent (Variables|Default|GetGlider) (Variables|Character|GetMesh) "gliderSocket" "KeepWorld" "KeepWorld" "KeepWorld" true)
  (Components|MoveComponentTo (Variables|Default|GetGlider) "0, 0, 0" "0, 0, 0" false false 0.2 false)
  (Transformation|SetRelativeScale3D (Variables|Default|GetGlider) "0.300000,0.200000,1.000000")
  (Variables|/Script/Engine.CharacterMovementComponent|SetGravityScale _charactermovement 1.0)
  (Variables|/Script/Engine.CharacterMovementComponent|SetMaxWalkSpeed _charactermovement 6e+02)
  (Transformation|AttachComponentToComponent (Variables|Default|GetFollowCamera) (Variables|Default|GetCameraBoom) "None" "KeepWorld" "KeepWorld" "KeepWorld" true)
  (Components|MoveComponentTo (Variables|Default|GetFollowCamera) "0, 0, 0" "0, 0, 0" false false 0.2 false))

(event Input|ActionEvents|InputActionDash
  (params (Key :type Key%20Structure :default "None"))
  (bind _returnvalue (Transformation|GetActorForwardVector))
  (bind _charactermovement (Variables|Character|GetCharacterMovement))
  (bind _inertiaforce (Variables|DashSettings|Inertia|GetinertiaForce))
  (bind _returnvalue_2 (* _returnvalue _inertiaforce))
  ;[1 1 1] Dash system
  ;;[1 1 1] Dash
  (:Pressed
    (if (Variables|DashSettings|Dash|GetCanDash)
      (bind _output_get (Variables|DashSettings|Private|SetstartDashPos (Transformation|GetActorLocation)))
      (Variables|DashSettings|Private|SetendDashPos (+ _output_get (* (Transformation|GetActorForwardVector) (Variables|DashSettings|Dash|GetdashDistance))))
      (bind _returnvalue_3 (Collision|LineTraceByChannel (Variables|DashSettings|Private|GetstartDashPos) (Variables|DashSettings|Private|GetendDashPos) "TraceTypeQuery1" false 0 "None"))
      (if (not _returnvalue_3)
        (Variables|DashSettings|Dash|SetCanDash false)
        (Components|MoveComponentTo (Variables|Default|GetCapsuleComponent) (Variables|DashSettings|Private|GetendDashPos) (Class|CharacterMovementComponent|GetLastUpdateRotation (Variables|Character|GetCharacterMovement)) false false (Variables|DashSettings|Dash|GetdashDuration) false)
        ;;[1 1 1] Inertia
        (if (AI|Components|NavMovement|IsFalling (Variables|Character|GetCharacterMovement))
          (Physics|AddImpulse (Variables|Character|GetCharacterMovement) _returnvalue_2 true)
          (Variables|/Script/Engine.CharacterMovementComponent|SetGroundFriction (Variables|Character|GetCharacterMovement) 0.0)
          (Variables|DashSettings|Private|SetdecreaseInertiaCooldown true)
          (else
            (Variables|/Script/Engine.CharacterMovementComponent|SetGroundFriction _charactermovement 0.0)
            (Physics|AddImpulse _charactermovement (* _returnvalue_2 1.7) true)
            (Variables|DashSettings|Private|SetdecreaseInertiaCooldown true)))
        (Utilities|FlowControl|Delay (Variables|DashSettings|Dash|GetdashCooldown))
        (Variables|DashSettings|Dash|SetCanDash true)))))

(event Input|ActionEvents|InputActionGlider
  (params (Key :type Key%20Structure :default "None"))
  (bind _charactermovement (Variables|Character|GetCharacterMovement))
  (bind _charactermovement_2 (Variables|Character|GetCharacterMovement))
  (bind _returnvalue (Pawn|Components|CharacterMovement|GetLastUpdateVelocity _charactermovement))
  ;[1 1 1] Glide system
  (:Pressed
    (if (Variables|GlideSettings|GetcanGlide)
      (if (Variables|GlideSettings|GetisGliding)
        (Variables|GlideSettings|SetisGliding false)
        (Transformation|AttachComponentToComponent (Variables|Default|GetGlider) (Variables|Character|GetMesh) "gliderSocket" "KeepWorld" "KeepWorld" "KeepWorld" true)
        (Components|MoveComponentTo (Variables|Default|GetGlider) "0, 0, 0" "0, 0, 0" false false 0.2 false)
        (Transformation|SetRelativeScale3D (Variables|Default|GetGlider) "0.300000,0.200000,1.000000")
        (Variables|/Script/Engine.CharacterMovementComponent|SetGravityScale _charactermovement_2 1.0)
        (Variables|/Script/Engine.CharacterMovementComponent|SetMaxWalkSpeed _charactermovement_2 6e+02)
        (Transformation|AttachComponentToComponent (Variables|Default|GetFollowCamera) (Variables|Default|GetCameraBoom) "None" "KeepWorld" "KeepWorld" "KeepWorld" true)
        (Components|MoveComponentTo (Variables|Default|GetFollowCamera) "0, 0, 0" "0, 0, 0" false false 0.2 false)
        (elif (AI|Components|NavMovement|IsFalling (Variables|Character|GetCharacterMovement))
          (Variables|GlideSettings|SetisGliding true)
          (Transformation|AttachComponentToComponent (Variables|Default|GetGlider) (Variables|Default|GetCapsuleComponent) "None" "KeepWorld" "KeepWorld" "KeepWorld" true)
          (Components|MoveComponentTo (Variables|Default|GetGlider) "0, 0,110.000000" "0, 0, 0" false false 0.2 false)
          (Transformation|SetRelativeScale3D (Variables|Default|GetGlider) "1.000000,1.000000,1.000000")
          (Variables|/Script/Engine.CharacterMovementComponent|SetGravityScale _charactermovement (Variables|GlideSettings|GetglidingGravityScale))
          (Variables|/Script/Engine.MovementComponent|SetVelocity _charactermovement (Math|Vector|MakeVector (.x _returnvalue) (.y _returnvalue) 0.0))
          (Variables|/Script/Engine.CharacterMovementComponent|SetMaxWalkSpeed (Variables|Character|GetCharacterMovement) (Variables|GlideSettings|GetmaxGlidingSpeed))
          (Transformation|AttachComponentToComponent (Variables|Default|GetFollowCamera) (Variables|Default|GetCameraBoom_gliding) "None" "KeepWorld" "KeepWorld" "KeepWorld" true)
          (Components|MoveComponentTo (Variables|Default|GetFollowCamera) "0, 0, 0" "0, 0, 0" false false 0.2 false))))))

(event Input|KeyboardEvents|Tab
  (params (Key :type Key%20Structure :default "None"))
  (bind _returnvalue (Game|GetPlayerController 0))
  (bind _globaltestui (Variables|Default|GetGlobalTestUI))
  ;[1 1 1] Press Tab to open/close settings widget
  (:Pressed
    (if (Widget|IsVisible (Variables|Default|GetGlobalTestUI))
      (Widget|SetVisibility _globaltestui "Hidden")
      (Variables|/Script/Engine.PlayerController|SetbShowMouseCursor _returnvalue false)
      (Variables|/Script/Engine.SpringArmComponent|SetbUsePawnControlRotation (Variables|Default|GetCameraBoom) true)
      (else
        (Widget|SetVisibility _globaltestui "Visible")
        (Variables|/Script/Engine.PlayerController|SetbShowMouseCursor _returnvalue true)
        (Variables|/Script/Engine.SpringArmComponent|SetbUsePawnControlRotation (Variables|Default|GetCameraBoom) false)))))

(event Input|MouseEvents|RightMouseButton
  (params (Key :type Key%20Structure :default "None"))
  (:Pressed
    (if (not (or false (Utilities|Enum|Equal(Enum) (Variables|PowerOption|GetUse%20Power%20Option) "NewEnumerator4")))
      (PowerOption|TryUsePower))))

(event Input|KeyboardEvents|T
  (params (Key :type Key%20Structure :default "None"))
  ;[1 1 1] Pickup Drop & Throw
  (:Pressed
    (if (Variables|PickupSettings|GetIsHolding?)
      (PickupSettings|Throw))))

(event Input|KeyboardEvents|E
  (params (Key :type Key%20Structure :default "None"))
  ;[1 1 1] Pickup Drop & Throw
  (:Pressed
    (if (Variables|PickupSettings|GetIsHolding?)
      (if (> (Math|Vector|VectorLength (Transformation|GetVelocity)) 0.0)
        (PickupSettings|Throw)
        (else
          (PickupSettings|Drop)))
      (else
        (Utilities|IsValid (Variables|PickupSettings|GetPickableObject)
          (:Is%20Valid
            (PickupSettings|Pickup)))))))

(event Input|KeyboardEvents|Tab
  (params (Key :type Key%20Structure :default "None"))
  ;[1 1 1] Press Tab to open/close settings widget
)

(event Input|KeyboardEvents|X
  (params (Key :type Key%20Structure :default "None"))
  (:Pressed
    (PowerOption|OnComboKeyInput Key)))

(event Input|KeyboardEvents|Y
  (params (Key :type Key%20Structure :default "None"))
  (:Pressed
    (PowerOption|OnComboKeyInput Key)))

(event Input|MouseEvents|LeftMouseButton
  (params (Key :type Key%20Structure :default "None"))
  ;[1 1 1] Get power in Buffer
  (:Pressed
    (if (and (Utilities|Enum|Equal(Enum) (Variables|PowerOption|GetGetPowerOption) "NewEnumerator1") (Utilities|Enum|NotEqual(Enum) (Variables|PowerOption|GetCurentAreaPower) "NewEnumerator0"))
      (PowerOption|ChangePower (Variables|PowerOption|GetCurentAreaPower)))))

(fn ConstructionScript)

(fn Pickup
  (bind _pickableobject (Variables|PickupSettings|GetPickableObject))
  (bind _cube (Variables|/Game/Blueprints/Pickup/PickupBP.PickupBP_C|GetCube _pickableobject))
  (Physics|SetSimulatePhysics _cube false)
  (Collision|SetCollisionEnabled _cube "NoCollision")
  (Transformation|AttachComponentToComponent _pickableobject (Variables|Default|GetPickupPoint) "None" "SnapToTarget" "KeepRelative" "KeepRelative" true)
  (Variables|PickupSettings|SetIsHolding? true)
  (Variables|PickupSettings|SetIs%20Picking%20Up? true)
  (Variables|PickupSettings|SetHolded%20Item _pickableobject)
  (Development|PrintString "Pick Up"))

(fn Drop
  (Transformation|DetachFromActor (Variables|PickupSettings|GetHolded%20Item) "KeepWorld" "KeepWorld" "KeepWorld")
  (Variables|PickupSettings|SetIsHolding? false)
  (Physics|SetSimulatePhysics (Variables|/Game/Blueprints/Pickup/PickupBP.PickupBP_C|GetCube (Variables|PickupSettings|GetHolded%20Item)) true)
  (Collision|SetCollisionEnabled (Variables|/Game/Blueprints/Pickup/PickupBP.PickupBP_C|GetCube (Variables|PickupSettings|GetHolded%20Item)) "QueryAndPhysics")
  (Variables|PickupSettings|SetHolded%20Item 0)
  (Development|PrintString "Drop"))

(fn CheckPickableObjects
  (bind _returnvalue (Transformation|GetActorLocation))
  (bind _returnvalue_2 (- _returnvalue "0, 0,40.000000"))
  (bind (_outhit _returnvalue_3) (Collision|LineTraceForObjects _returnvalue_2 (+ _returnvalue_2 (* (Transformation|GetActorForwardVector) 1e+02)) (Utilities|Array|MakeArray "ObjectTypeQuery7") false 0 "ForOneFrame"))
  (if _returnvalue_3
    (bind _aspickup_bp (Utilities|Casting|CastToPickupBP (.HitActor (Collision|BreakHitResult _outhit)))
      (:then
        (if (not (== _aspickup_bp (Variables|PickupSettings|GetPickableObject)))
          (Variables|PickupSettings|SetPickableObject _aspickup_bp)
          (Utilities|IsValid (Variables|PickupSettings|GetPickup%20Widget)
            (:Is%20Valid
              _)
            (:Is%20Not%20Valid
              (bind _returnvalue_4 (UserInterface|CreateWidget "/Game/Assets/GPAssets/Widget/PickupWidget.PickupWidget_C"))
              (bind _output_get (Variables|PickupSettings|SetPickup%20Widget _returnvalue_4))))
          (UserInterface|Viewport|AddtoViewport _output_get 0)))
      (:CastFailed
        (Utilities|IsValid (Variables|PickupSettings|GetPickableObject) :!label _label
          (:Is%20Valid
            (Variables|PickupSettings|SetPickableObject 0)
            (Utilities|IsValid (Variables|PickupSettings|GetPickup%20Widget)
              (:Is%20Valid
                (Widget|RemovefromParent (Variables|PickupSettings|GetPickup%20Widget))))))))
    (else
      (goto _label))))

(fn Throw
  (Transformation|DetachFromActor (Variables|PickupSettings|GetHolded%20Item) "KeepWorld" "KeepWorld" "KeepWorld")
  (Variables|PickupSettings|SetIsHolding? false)
  (Physics|SetSimulatePhysics (Variables|/Game/Blueprints/Pickup/PickupBP.PickupBP_C|GetCube (Variables|PickupSettings|GetHolded%20Item)) true)
  (Collision|SetCollisionEnabled (Variables|/Game/Blueprints/Pickup/PickupBP.PickupBP_C|GetCube (Variables|PickupSettings|GetHolded%20Item)) "QueryAndPhysics")
  (Physics|AddImpulse (Variables|/Game/Blueprints/Pickup/PickupBP.PickupBP_C|GetCube (Variables|PickupSettings|GetHolded%20Item)) (* (+ (Transformation|GetActorForwardVector) "0, 0,1.000000") (Variables|PickupSettings|GetThrowForce)) "None" true)
  (Variables|PickupSettings|SetHolded%20Item 0)
  (Development|PrintString "Throw"))

(fn ChangePower
  (params (NewPower :type PowerEnum%20Enum :default "NewEnumerator0"))
  (bind _mainpowerparticle (Variables|Default|GetMainPowerParticle))
  (Variables|PowerOption|SetLastPower (Variables|PowerOption|GetCurrentPower))
  (Variables|PowerOption|SetCurrentPower NewPower)
  (PowerOption|ClearTimer)
  (if (Utilities|Enum|Equal(Enum) (Variables|PowerOption|GetUsePowerOption) "NewEnumerator4")
    (PowerOption|TryUsePower)
    (else
      (Utilities|FlowControl|Sequence
        (:then_0
          (switch Utilities|FlowControl|Switch|SwitchonPowerEnum (Variables|PowerOption|GetCurrentPower)
            (:NewEnumerator0
              (Effects|Components|ParticleSystem|SetEmitterEnable _mainpowerparticle "Particle Emitter" false))
            (:NewEnumerator1
              (Effects|Components|ParticleSystem|SetColorParameter _mainpowerparticle "Color" "(R=1.000000,G=0.000000,B=0.000000,A=1.000000)")
              (Effects|Components|ParticleSystem|SetEmitterEnable _mainpowerparticle "Particle Emitter" true :!label _label))
            (:NewEnumerator2
              (Effects|Components|ParticleSystem|SetColorParameter _mainpowerparticle "Color" "(R=0.000000,G=0.000000,B=1.000000,A=1.000000)")
              (goto _label))))))))

(fn OnComboKeyInput
  (params (Input :type Key%20Structure :default "None"))
  (if (== Input (Utilities|Array|Get(acopy) (Variables|PowerOption|GetComboKeys) (Variables|PowerOption|GetCurrentKeyIndex)))
    (bind _result (Math|Integer|IncrementInt (Variables|PowerOption|GetCurrentKeyIndex))
      (:%20%20
        (Audio|PlaySound2D "/Game/Sounds/Sounds/Collectible.Collectible" 1.0 (+ (/ (Math|Conversions|ToFloat(Integer) (Variables|PowerOption|GetCurrentKeyIndex)) (Math|Conversions|ToFloat(Integer) (Utilities|Array|Length (Variables|PowerOption|GetComboKeys)))) 1.0) 0.2 0 0)
        (if (<= (Utilities|Array|Length (Variables|PowerOption|GetComboKeys)) _result)
          ;[1 1 1] Combo Success
          (Variables|PowerOption|SetCurrentKeyIndex 0)
          (if (Utilities|Enum|Equal(Enum) (Variables|PowerOption|GetGetPowerOption) "NewEnumerator3")
            (PowerOption|ChangePower (Variables|PowerOption|GetCurentAreaPower))
            (elif (and (Variables|PowerOption|GetUseWithCombo) (Utilities|Enum|NotEqual(Enum) (Variables|PowerOption|GetUsePowerOption) "NewEnumerator4"))
              (PowerOption|TryUsePower)))
          (else
            (PowerOption|StartComboTimer)))))
    (else
      (PowerOption|ComboFail)
      (Audio|PlaySound2D "/Game/Sounds/Sounds/WrongKey.WrongKey" 1.0 1.0 0.2 0 0))))

(fn TryUsePower
  (if (and (Utilities|Enum|NotEqual(Enum) (Variables|PowerOption|GetCurrentPower) "NewEnumerator0") true)
    (switch Utilities|FlowControl|Switch|SwitchonPowerEnum (Variables|PowerOption|GetCurrentPower)
      (:NewEnumerator1
        (Game|SpawnActorfromClass "/Game/Blueprints/PowerAreaBP/SpawnableWall.SpawnableWall_C" (Transformation|GetActorTransform) "AlwaysSpawn" 0 0))
      (:NewEnumerator2
        (Game|SpawnActorfromClass "/Game/Blueprints/PowerAreaBP/Sphere_Blue.Sphere_Blue_C" (Math|Conversions|ToTransform(Vector) (+ (Transformation|GetActorLocation) (* (Transformation|GetActorForwardVector) 1e+02))) "AlwaysSpawn" 0 0)))
    (if (and (Utilities|Enum|Equal(Enum) (Variables|PowerOption|GetUsePowerOption) "NewEnumerator0") (or (and (Utilities|Enum|Equal(Enum) (Variables|PowerOption|GetGetPowerOption) "NewEnumerator0") (Utilities|Enum|NotEqual(Enum) (Variables|PowerOption|GetCurrentPower) (Variables|PowerOption|GetCurentAreaPower))) (Utilities|Enum|NotEqual(Enum) (Variables|PowerOption|GetGetPowerOption) "NewEnumerator0")))
      (PowerOption|RemovePower))))

(fn ClearTimer
  (bind _timer (Variables|PowerOption|GetTimer))
  (if (Utilities|Time|IsValidTimerHandle _timer)
    (Utilities|Time|ClearandInvalidateTimerbyHandle _timer)))

(fn ComboFail
  (Utilities|Time|ClearandInvalidateTimerbyHandle (Variables|PowerOption|GetComboTimer))
  (Development|PrintString "Combo Failled")
  (Variables|PowerOption|SetCurrentKeyIndex 0))

(fn StartComboTimer
  (if (Utilities|Time|IsValidTimerHandle (Variables|PowerOption|GetComboTimer))
    (Utilities|Time|ClearandInvalidateTimerbyHandle (Variables|PowerOption|GetComboTimer)))
  (bind _returnvalue (Utilities|Time|SetTimerbyFunctionName self "ComboFail" (Variables|PowerOption|GetTimeBetweenCombo)))
  (Variables|PowerOption|SetComboTimer _returnvalue))

(fn RemovePower
  (Variables|PowerOption|SetCurrentPower "NewEnumerator0")
  (Variables|PowerOption|SetLastPower "NewEnumerator0")
  (Development|PrintString "Power Removed")
  (Effects|Components|ParticleSystem|SetEmitterEnable (Variables|Default|GetMainPowerParticle) "Particle Emitter" false))

(fn EnterPowerArea
  (params (ZoneType :type PowerEnum%20Enum :default "NewEnumerator0"))
  (Variables|PowerOption|SetCurentAreaPower ZoneType)
  (switch Utilities|FlowControl|Switch|SwitchonPowerGetEnum (Variables|PowerOption|GetGetPowerOption)
    (:NewEnumerator0
      (PowerOption|ChangePower (Variables|PowerOption|GetCurentAreaPower)))))

(fn ExitPowerArea
  (params (ZoneType :type PowerEnum%20Enum :default "NewEnumerator0"))
  (if (Utilities|Enum|Equal(Enum) ZoneType (Variables|PowerOption|GetCurentAreaPower))
    (Variables|PowerOption|SetCurentAreaPower "NewEnumerator0")
    (switch Utilities|FlowControl|Switch|SwitchonPowerLoseEnum (Variables|PowerOption|GetLosePowerOption)
      (:NewEnumerator0
        (PowerOption|RemovePower))
      (:NewEnumerator2
        (bind _returnvalue (Utilities|Time|SetTimerbyFunctionName self "RemovePower" (Variables|PowerOption|GetLosePowerCooldown)))
        (Variables|PowerOption|SetTimer _returnvalue)))))