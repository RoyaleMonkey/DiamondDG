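; GlobalGameMode is a game mode that handles respawning and owns a test UI widget.
; BeginPlay caches the PlayerStart transform as the respawn point and creates a hidden GlobalTestWidget in the viewport.
; Tick polls player 0's pawn and, when none is valid, spawns a GlobalCharacter at that point, has that character's own controller possess it, then calls LoadSave on the widget.
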(event EventBeginPlay
  (bind _returnvalue (Actor|GetActorOfClass "/Script/Engine.PlayerStart"))
  (Variables|Default|SetRespawnPoint (Transformation|GetActorTransform _returnvalue))
  (bind _returnvalue_2 (UserInterface|CreateWidget "/Game/Assets/GPAssets/Widget/GlobalTestWidget.GlobalTestWidget_C"))
  (UserInterface|Viewport|AddtoViewport _returnvalue_2 1)
  (Widget|SetVisibility _returnvalue_2 "Hidden")
  (Variables|Default|SetGlobalTestUI _returnvalue_2))

(event EventTick
  (params (DeltaSeconds :type Float%20%28single-precision%29))
  (bind _respawnpoint (Variables|Default|GetRespawnPoint))
  (if (not (Utilities|IsValid (Pawn|GetControlledPawn (Game|GetPlayerController 0))))
    (bind _returnvalue (Game|SpawnActorfromClass "/Game/Blueprints/Character/GlobalCharacter.GlobalCharacter_C" (Math|Transform|MakeTransform (.location _respawnpoint) (.rotation _respawnpoint) "1,1,1") "Undefined" 0 0))
    (Pawn|Possess (Pawn|GetController _returnvalue) _returnvalue)
    (Default|LoadSave (Variables|Default|GetGlobalTestUI))))

(fn ConstructionScript)