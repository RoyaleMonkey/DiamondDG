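; Character component that runs a tempo-based input combo, judging whether key presses land within a margin around each beat.
; Tick advances the beat timer while activated and plays force feedback shortly before each beat; the timer only resets once that vibration has triggered.
; On-beat input sustains the combo and calls loop start when the index passes the list's end.
; Off-beat or missed input plays a wrong-key sound and calls loop end.
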(event EventTick
  (params (DeltaSeconds :type Float%20%28single-precision%29))
  (Utilities|FlowControl|Sequence
    (:then_0
      ;[1 1 1] TempoVibration
      (if (Variables|Default|GetActivated)
        (bind _output_get (Variables|Default|SetTempoTimer (+ (Variables|Default|GetTempoTimer) DeltaSeconds)))
        (if (> _output_get (- (Variables|Default|GetTempo) (Variables|Default|GetVibrationOffset)))
          (if (not (Variables|Default|GetVibrationActivated))
            (if (Variables|Default|GetShouldVibrate)
              (Game|Feedback|ClientPlayForceFeedback (Game|GetPlayerController 0) "/Game/Blueprints/Character/CustomParam/TempoVibration.TempoVibration" "None" false false false)
              (Variables|Default|SetVibrationActivated true))
            (elif (> (Variables|Default|GetTempoTimer) (Variables|Default|GetTempo))
              (Variables|Default|SetTempoTimer 0.0)
              (Variables|Default|SetVibrationActivated false))))))
    (:then_1
      ;[1 1 1] StopCombo if no key
      (if (Math|Boolean|ANDBoolean (Variables|Default|GetComboStart) (not (Variables|Default|GetComboValidate)) (> (Variables|Default|GetTempoTimer) (Variables|Default|GetMargin)) (< (Variables|Default|GetTempoTimer) (- (Variables|Default|GetTempo) (Variables|Default|GetMargin))))
        (if (not (Variables|Default|GetComboContinue))
          (Variables|Default|SetComboStart false)
          (Audio|PlaySound2D "/Game/Sounds/Sounds/WrongKey.WrongKey" 1.0 1.0 0.0 0 0)
          (Default|CallOnLoopEnd)
          (else
            (Variables|Default|SetComboValidate true)
            (Variables|Default|SetComboContinue false)))))
    (:then_2
      (if (and (> (Variables|Default|GetTempoTimer) (- (Variables|Default|GetTempo) (Variables|Default|GetMargin))) (Variables|Default|GetComboValidate))
        (Variables|Default|SetComboValidate false)))))

(fn InputReceived
  (params (Index :type Integer%20%28by%20ref%29) (List :type Array%20of%20ComboInput%20Enums :default "NewEnumerator0"))
  (if (or (> (Variables|Default|GetTempoTimer) (- (Variables|Default|GetTempo) (Variables|Default|GetMargin))) (< (Variables|Default|GetTempoTimer) (Variables|Default|GetMargin)))
    (Variables|Default|SetComboStart true)
    (Variables|Default|SetComboContinue true)
    (if (>= Index (Utilities|Array|Length List))
      (|SetBy-RefVar Index)
      (Default|CallOnLoopStart))
    (else
      (Audio|PlaySound2D "/Game/Sounds/Sounds/WrongKey.WrongKey" 1.0 1.0 0.0 0 0)
      (Variables|Default|SetComboStart false)
      (|SetBy-RefVar Index)
      (Default|CallOnLoopEnd))))