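; Test character for a power-area mechanic: it gains, uses and loses colored powers from zones, with configurable rules and a debug widget toggled by Tab.
; Zone enter/exit tracks the area's power, granted on trigger, left click or timed X/Y combo.
; Right click or combo uses power, printing it and optionally consuming it.
; Loss can be immediate or timer-delayed on exit; a particle emitter shows the current color.
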(event EventBeginPlay
  ;[1 1 1] Begin play
  (Effects|Components|ParticleSystem|SetEmitterEnable (Variables|Default|GetMainPowerParticle) "Particle Emitter" false)
  (Effects|Components|ParticleSystem|SetEmitterEnable (Variables|Default|GetSecondPowerParticle) "Particle Emitter" false)
  (bind _returnvalue (UserInterface|CreateWidget "/Game/Assets/GPAssets/Widget/TestPowerArea.TestPowerArea_C"))
  (UserInterface|Viewport|AddtoViewport _returnvalue 0)
  (Variables|Default|Setwidget _returnvalue))

(event Input|MouseEvents|LeftMouseButton
  (params (Key :type Key%20Structure :default "None"))
  ;[1 1 1] Get power in Buffer
  (:Pressed
    (if (and (Utilities|Enum|Equal(Enum) (Variables|PowerOption|GetGetPowerOption) "NewEnumerator1") (Utilities|Enum|NotEqual(Enum) (Variables|privateVar|GetCurentAreaPower) "NewEnumerator0"))
      (CallFunction|ChangePower (Variables|privateVar|GetCurentAreaPower)))))

(event Input|MouseEvents|RightMouseButton
  (params (Key :type Key%20Structure :default "None"))
  (:Pressed
    (if (not (Variables|PowerOption|GetUseWithCombo))
      (CallFunction|TryUsePower))))

(event Input|KeyboardEvents|Tab
  (params (Key :type Key%20Structure :default "None"))
  (bind _returnvalue (Game|GetPlayerController 0))
  (bind _returnvalue_2 (Game|GetPlayerController 0))
  ;[1 1 1] Ui interaction
  (:Pressed
    (if (Variables|privateVar|GetUIMode?)
      (Input|SetInputModeGameOnly _returnvalue_2)
      (Variables|/Script/Engine.PlayerController|SetbShowMouseCursor _returnvalue false)
      (Variables|privateVar|SetUIMode? false)
      (else
        (Input|SetInputModeGameandUI _returnvalue_2 (Variables|Default|Getwidget) "DoNotLock" true)
        (Variables|/Script/Engine.PlayerController|SetbShowMouseCursor _returnvalue true)
        (Variables|privateVar|SetUIMode? true)))))

(event Input|KeyboardEvents|X
  (params (Key :type Key%20Structure :default "None"))
  (:Pressed
    (CallFunction|OnComboKeyInput Key)))

(event Input|KeyboardEvents|Y
  (params (Key :type Key%20Structure :default "None"))
  (:Pressed
    (CallFunction|OnComboKeyInput Key)))

(fn ConstructionScript)

(fn EnterPowerArea
  (params (ZoneType :type PowerEnum%20Enum :default "NewEnumerator0"))
  (Variables|privateVar|SetCurentAreaPower ZoneType)
  (switch Utilities|FlowControl|Switch|SwitchonPowerGetEnum (Variables|PowerOption|GetGetPowerOption)
    (:NewEnumerator0
      (CallFunction|ChangePower (Variables|privateVar|GetCurentAreaPower)))))

(fn ExitPowerArea
  (params (ZoneType :type PowerEnum%20Enum :default "NewEnumerator0"))
  (if (Utilities|Enum|Equal(Enum) ZoneType (Variables|privateVar|GetCurentAreaPower))
    (Variables|privateVar|SetCurentAreaPower "NewEnumerator0")
    (switch Utilities|FlowControl|Switch|SwitchonPowerLoseEnum (Variables|PowerOption|GetLosePowerOption)
      (:NewEnumerator0
        (CallFunction|RemovePower))
      (:NewEnumerator2
        (bind _returnvalue (Utilities|Time|SetTimerbyFunctionName self "RemovePower" (Variables|PowerOption|GetLosePowerCooldown)))
        (Variables|privateVar|SetTimer _returnvalue)))))

(fn RemovePower
  (Variables|privateVar|SetCurrentPower "NewEnumerator0")
  (Variables|privateVar|SetLastPower "NewEnumerator0")
  (Development|PrintString "Power Removed")
  (Effects|Components|ParticleSystem|SetEmitterEnable (Variables|Default|GetMainPowerParticle) "Particle Emitter" false))

(fn ChangePower
  (params (NewPower :type PowerEnum%20Enum :default "NewEnumerator0"))
  (bind _mainpowerparticle (Variables|Default|GetMainPowerParticle))
  (Variables|privateVar|SetLastPower (Variables|privateVar|GetCurrentPower))
  (Variables|privateVar|SetCurrentPower NewPower)
  (CallFunction|ClearTimer)
  (Utilities|FlowControl|Sequence
    (:then_0
      (switch Utilities|FlowControl|Switch|SwitchonPowerEnum (Variables|privateVar|GetCurrentPower)
        (:NewEnumerator0
          (Effects|Components|ParticleSystem|SetEmitterEnable _mainpowerparticle "Particle Emitter" false))
        (:NewEnumerator1
          (Effects|Components|ParticleSystem|SetColorParameter _mainpowerparticle "Color" "(R=1.000000,G=0.000000,B=0.000000,A=1.000000)")
          (Effects|Components|ParticleSystem|SetEmitterEnable _mainpowerparticle "Particle Emitter" true :!label _label))
        (:NewEnumerator2
          (Effects|Components|ParticleSystem|SetColorParameter _mainpowerparticle "Color" "(R=0.000000,G=0.000000,B=1.000000,A=1.000000)")
          (goto _label))))))

(fn ClearTimer
  (bind _timer (Variables|privateVar|GetTimer))
  (if (Utilities|Time|IsValidTimerHandle _timer)
    (Utilities|Time|ClearandInvalidateTimerbyHandle _timer)))

(fn OnComboKeyInput
  (params (Input :type Key%20Structure :default "None"))
  (if (== Input (Utilities|Array|Get(acopy) (Variables|PowerOption|GetComboKeys) (Variables|privateVar|GetCurrentKeyIndex)))
    (bind _result (Math|Integer|IncrementInt (Variables|privateVar|GetCurrentKeyIndex))
      (:%20%20
        (if (<= (Utilities|Array|Length (Variables|PowerOption|GetComboKeys)) _result)
          ;[1 1 1] Combo Success
          (if (Utilities|Enum|Equal(Enum) (Variables|PowerOption|GetGetPowerOption) "NewEnumerator3")
            (CallFunction|ChangePower (Variables|privateVar|GetCurentAreaPower))
            (elif (Variables|PowerOption|GetUseWithCombo)
              (CallFunction|TryUsePower)))
          (else
            (CallFunction|StartComboTimer)))))
    (else
      (CallFunction|ComboFail))))

(fn ComboFail
  (Utilities|Time|ClearandInvalidateTimerbyHandle (Variables|privateVar|GetComboTimer))
  (Development|PrintString "Combo Failled")
  (Variables|privateVar|SetCurrentKeyIndex 0))

(fn StartComboTimer
  (if (Utilities|Time|IsValidTimerHandle (Variables|privateVar|GetComboTimer))
    (Utilities|Time|ClearandInvalidateTimerbyHandle (Variables|privateVar|GetComboTimer)))
  (bind _returnvalue (Utilities|Time|SetTimerbyFunctionName self "ComboFail" (Variables|PowerOption|GetTimeBetweenCombo)))
  (Variables|privateVar|SetComboTimer _returnvalue))

(fn TryUsePower
  ;[1 1 1] Use Power
  (Development|PrintString (Utilities|String|EnumtoString (Variables|privateVar|GetCurrentPower)))
  (if (and (Utilities|Enum|Equal(Enum) (Variables|PowerOption|GetUsePowerOption) "NewEnumerator0") (or (and (Utilities|Enum|Equal(Enum) (Variables|PowerOption|GetGetPowerOption) "NewEnumerator0") (Utilities|Enum|NotEqual(Enum) (Variables|privateVar|GetCurrentPower) (Variables|privateVar|GetCurentAreaPower))) (Utilities|Enum|NotEqual(Enum) (Variables|PowerOption|GetGetPowerOption) "NewEnumerator0")))
    (CallFunction|RemovePower)))