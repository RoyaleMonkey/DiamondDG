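; Actor component that gives its owner a timed slow-motion ability, slowing the world while the owner keeps normal speed.
; LaunchSlowSphere, guarded against re-triggering while active, sets global time dilation to SlowRatio and gives the owner the inverse custom dilation.
; A timer scaled by SlowRatio keeps the duration in real seconds, then calls UnSlowActors to restore global, owner and player camera manager dilation and clear the state.
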(event EventBeginPlay)

(event EventTick
  (params (DeltaSeconds :type Float%20%28single-precision%29)))

(fn UnSlowActors
  (Utilities|Time|SetGlobalTimeDilation 1.0)
  (Variables|/Script/Engine.Actor|SetCustomTimeDilation (Components|GetOwner) 1.0)
  (Variables|/Script/Engine.Actor|SetCustomTimeDilation (Variables|/Script/Engine.PlayerController|GetPlayerCameraManager (Game|GetPlayerController 0)) 1.0)
  (Utilities|Time|ClearandInvalidateTimerbyHandle (Variables|Default|GetSlow%20Timer))
  (Variables|Default|SetisActive? false))

(fn LaunchSlowSphere
  (bind _slowratio (Variables|Default|GetSlowRatio))
  (if (not (or (Variables|Default|GetisActive?) (Utilities|Time|IsTimerActivebyHandle (Variables|Default|GetSlow%20Timer))))
    (Variables|Default|SetisActive? true)
    (Utilities|Time|SetGlobalTimeDilation _slowratio)
    (Variables|/Script/Engine.Actor|SetCustomTimeDilation (Components|GetOwner) (/ 1.0 _slowratio))
    (bind _returnvalue (Utilities|Time|SetTimerbyFunctionName self "UnSlowActors" (* (Variables|Default|GetSlowDuration) (Variables|Default|GetSlowRatio))))
    (Variables|Default|SetSlow%20Timer _returnvalue)))