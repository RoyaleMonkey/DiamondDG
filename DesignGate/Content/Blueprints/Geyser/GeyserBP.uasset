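; Geyser actor that launches the player character and physics-simulating objects along its ground visual's up vector.
; BeginPlay scales the trigger's height, optionally destroys the geyser after a lifetime, and starts a ChangeState timer that can switch the particle emitter off.
; Tick applies impulses to overlapping actors regardless of active state, also dezooming the player's camera.
; Objects need a simulating static mesh root, and the AutoGlide call is unwired.
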(event Custom|ChangeState
  ;[1 1 1] Particle emitter
  (bind _output_get (Variables|Default|SetisActive (not (Variables|Default|GetisActive))))
  (if (not _output_get)
    (Effects|Components|ParticleSystem|SetEmitterEnable (Variables|Default|GetParticleSystem) "Particle" _output_get)
    (Utilities|Time|SetTimerbyEvent (delegate Custom|ChangeState) (Math|Float|SelectFloat (Variables|Geysersettings|GetactivationTime) (Variables|Geysersettings|GetdisableTime) _output_get))))

(event Custom|Character
  (params (overlapedActor :type Actor%20Object%20Reference))
  ;[1 1 1] Character projection
  (bind _asglobal_character (Utilities|Casting|CastToGlobalCharacter overlapedActor))
  (Default|CamDezoom _asglobal_character)
  (Physics|AddImpulse (Variables|/Script/Engine.Character|GetCharacterMovement _asglobal_character) (* (Math|Vector|GetUpVector (Variables|Default|GetGroundVisual)) (* 1e+01 (Variables|Geysersettings|GetthrowPlayerForce))) false))

(event Custom|Object%20projection
  (params (overlapedActor :type Actor%20Object%20Reference))
  (bind _rootcomponent (Variables|/Script/Engine.Actor|GetRootComponent overlapedActor))
  ;[1 1 1] Object projection
  (if (Physics|IsSimulatingPhysics _rootcomponent "None")
    ;;[1 1 1] Maybe change to promitive component
    (bind _asstatic_mesh_component (Utilities|Casting|CastToStaticMeshComponent _rootcomponent))
    (Physics|AddImpulse _asstatic_mesh_component (* (Math|Vector|GetUpVector (Variables|Default|GetGroundVisual)) (* 1e+01 (Variables|Geysersettings|GetthrowObjectForce))) "None" false)))

(event EventTick
  (params (DeltaSeconds :type Float%20%28single-precision%29))
  ;[1 1 1] Check overlapped actors
  (for _array_element (Collision|GetOverlappingActors (Variables|Default|GetTrigger) 0 :!class /Script/Engine.PrimitiveComponent)
    (if (== _array_element (Game|GetPlayerCharacter 0))
      (CallFunction|Character _array_element)
      (else
        (CallFunction|ObjectProjection _array_element)))))

(event EventBeginPlay
  (bind _trigger (Variables|Default|GetTrigger))
  (bind _returnvalue (Transformation|GetWorldScale _trigger))
  ;[1 1 1] Set geyser max height & lifetime
  (Utilities|FlowControl|Sequence
    (:then_0
      (Transformation|SetWorldScale3D _trigger (Math|Vector|MakeVector (.x _returnvalue) (.y _returnvalue) (Variables|Geysersettings|GettriggerScale)))
      (if (not (== 0.0 (Variables|Geysersettings|GetgeyserLifetime)))
        (Utilities|FlowControl|Delay (Variables|Geysersettings|GetgeyserLifetime))
        (Actor|DestroyActor)))
    (:then_1
      ;[1 1 1] Particle emitter
      (Utilities|Time|SetTimerbyEvent (delegate Custom|ChangeState) (Variables|Geysersettings|GetdisableTime)))))

(fn ConstructionScript)