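; Pickup actor that the player's GlobalCharacter can carry, drop or throw through Interact.
; Pickup disables physics and collision, attaches the actor to the character's PickupPoint and records it as the held item.
; Interacting while holding throws if the character is moving, otherwise drops, restoring physics and collision.
; Throws add a mass-independent forward-and-up impulse scaled by the character's ThrowForce.
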(event EventBeginPlay
  (bind _asglobal_character (Utilities|Casting|CastToGlobalCharacter (Game|Player|GetPlayerPawn 0)))
  (Variables|Default|SetGlobalCharacter _asglobal_character))

(fn ConstructionScript)

(fn Interact
  (if (Variables|/Game/Blueprints/Character/GlobalCharacter.GlobalCharacter_C|GetIsHolding? (Variables|Default|GetGlobalCharacter))
    (if (> (Math|Vector|VectorLength (Transformation|GetVelocity (Variables|Default|GetGlobalCharacter))) 0.0)
      (CallFunction|Throw)
      (else
        (CallFunction|Drop)))
    (else
      (CallFunction|Pickup))))

(fn Pickup
  (bind _staticmeshcomponent (Variables|Default|GetStaticMeshComponent))
  (bind _globalcharacter (Variables|Default|GetGlobalCharacter))
  (Physics|SetSimulatePhysics _staticmeshcomponent false)
  (Collision|SetCollisionEnabled _staticmeshcomponent "NoCollision")
  (Transformation|AttachComponentToComponent self (Variables|/Game/Blueprints/Character/GlobalCharacter.GlobalCharacter_C|GetPickupPoint (Variables|Default|GetGlobalCharacter)) "None" "SnapToTarget" "KeepWorld" "KeepWorld" true)
  (Variables|/Game/Blueprints/Character/GlobalCharacter.GlobalCharacter_C|SetIsHolding? _globalcharacter true)
  (Variables|/Game/Blueprints/Character/GlobalCharacter.GlobalCharacter_C|SetIs%20Picking%20Up? _globalcharacter true)
  (Variables|/Game/Blueprints/Character/GlobalCharacter.GlobalCharacter_C|SetHolded%20Item _globalcharacter self))

(fn Drop
  (bind _globalcharacter (Variables|Default|GetGlobalCharacter))
  (bind _staticmeshcomponent (Variables|Default|GetStaticMeshComponent))
  (Transformation|DetachFromActor self "KeepWorld" "KeepWorld" "KeepWorld")
  (Variables|/Game/Blueprints/Character/GlobalCharacter.GlobalCharacter_C|SetIsHolding? _globalcharacter false)
  (Physics|SetSimulatePhysics _staticmeshcomponent true)
  (Collision|SetCollisionEnabled _staticmeshcomponent "QueryAndPhysics")
  (Variables|/Game/Blueprints/Character/GlobalCharacter.GlobalCharacter_C|SetHolded%20Item _globalcharacter 0))

(fn Throw
  (bind _globalcharacter (Variables|Default|GetGlobalCharacter))
  (bind _globalcharacter_2 (Variables|Default|GetGlobalCharacter))
  (bind _staticmeshcomponent (Variables|Default|GetStaticMeshComponent))
  (Transformation|DetachFromActor self "KeepWorld" "KeepWorld" "KeepWorld")
  (Variables|/Game/Blueprints/Character/GlobalCharacter.GlobalCharacter_C|SetIsHolding? _globalcharacter_2 false)
  (Physics|SetSimulatePhysics _staticmeshcomponent true)
  (Collision|SetCollisionEnabled _staticmeshcomponent "QueryAndPhysics")
  (Physics|AddImpulse _staticmeshcomponent (* (+ (Transformation|GetActorForwardVector _globalcharacter) "0, 0,1.000000") (Variables|/Game/Blueprints/Character/GlobalCharacter.GlobalCharacter_C|GetThrowForce _globalcharacter)) "None" true)
  (Variables|/Game/Blueprints/Character/GlobalCharacter.GlobalCharacter_C|SetHolded%20Item _globalcharacter_2 0))