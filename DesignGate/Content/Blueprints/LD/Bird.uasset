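; Level-design actor that flies a bird along a spline trajectory in a repeating loop.
; After a start delay, Tick calls MakeFly, which advances the distance by speed and aligns the bird to the spline with a yaw offset.
; A dynamic material's opacity fades the bird in and out near both ends of the path.
; At the end, flight stops and Restart resets the distance after a delay.
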(event Custom|Restart
  (Utilities|FlowControl|Delay (Variables|Default|GetDelayBetweenLoop))
  (Variables|Default|SetCurrentDistanceOnTrajectory 0.0)
  (Variables|Default|SetIsFlying true))

(event EventBeginPlay
  (bind _returnvalue (Rendering|Material|CreateDynamicMaterialInstance (Variables|Default|GetBird) 0 0 "None" :!class /Script/Engine.PrimitiveComponent))
  (bind _output_get (Variables|Default|SetMaterialInstance _returnvalue))
  (Rendering|Material|SetScalarParameterValue _output_get "Opacity" 0.0 :!class /Script/Engine.MaterialInstanceDynamic)
  (Utilities|FlowControl|Delay (Variables|Default|GetStartDelay))
  (Variables|Default|SetIsFlying true))

(event EventTick
  (params (DeltaSeconds :type Float%20%28single-precision%29))
  (CallFunction|MakeFly DeltaSeconds))

(fn ConstructionScript)

(fn MakeFly
  (params (DeltaSeconds :type Float%20%28single-precision%29))
  (bind _trajectory (Variables|Default|GetTrajectory))
  (if (Variables|Default|GetIsFlying)
    (bind _output_get (Variables|Default|SetCurrentDistanceOnTrajectory (Math|Float|Min(Float) (+ (Variables|Default|GetCurrentDistanceOnTrajectory) (* DeltaSeconds (Variables|Default|GetSpeed) 1e+02)) (Spline|GetSplineLength (Variables|Default|GetTrajectory)))))
    (Transformation|SetWorldLocationAndRotation (Variables|Default|GetBird) (Spline|GetLocationatDistanceAlongSpline _trajectory _output_get "World") (Math|Rotator|MakeRotator (.roll (Spline|GetRotationatDistanceAlongSpline _trajectory _output_get "World")) (.pitch (Spline|GetRotationatDistanceAlongSpline _trajectory _output_get "World")) (- (.yaw (Spline|GetRotationatDistanceAlongSpline _trajectory _output_get "World")) 9e+01)) false false)
    (if (or (<= (Variables|Default|GetCurrentDistanceOnTrajectory) (Variables|Default|GetFadeInAndOutDistance)) (<= (- (Spline|GetSplineLength (Variables|Default|GetTrajectory)) (Variables|Default|GetCurrentDistanceOnTrajectory)) (Variables|Default|GetFadeInAndOutDistance)))
      (Rendering|Material|SetScalarParameterValue (Variables|Default|GetMaterialInstance) "Opacity" (Math|Float|Lerp 0.0 1.0 (/ (Math|Float|SelectFloat (Variables|Default|GetCurrentDistanceOnTrajectory) (- (Spline|GetSplineLength (Variables|Default|GetTrajectory)) (Variables|Default|GetCurrentDistanceOnTrajectory)) (<= (Variables|Default|GetCurrentDistanceOnTrajectory) (Variables|Default|GetFadeInAndOutDistance))) (Variables|Default|GetFadeInAndOutDistance))) :!class /Script/Engine.MaterialInstanceDynamic))
    (if (== (Variables|Default|GetCurrentDistanceOnTrajectory) (Spline|GetSplineLength (Variables|Default|GetTrajectory)))
      (Variables|Default|SetIsFlying false)
      (CallFunction|Restart))))