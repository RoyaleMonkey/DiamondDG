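; Level-design checkpoint that sets the player's respawn point and saves the game when a GlobalCharacter enters its trigger box.
; BeginPlay caches the GlobalGameMode, and an overlap while active copies the RespawnPoint component's world transform into it.
; The checkpoint then deactivates unless ForeverActive is set, and calls the character's SaveGame with that transform at unit scale.
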(event OnComponentBeginOverlap(TriggerBox)
  (params (OverlappedComponent :type Primitive%20Component%20Object%20Reference) (OtherActor :type Actor%20Object%20Reference) (OtherComp :type Primitive%20Component%20Object%20Reference) (OtherBodyIndex :type Integer) (bFromSweep :type Boolean) (SweepResult :type Hit%20Result%20Structure%20%28by%20ref%29))
  (bind _asglobal_character (Utilities|Casting|CastToGlobalCharacter OtherActor))
  (if (Variables|Default|GetIsActive)
    (bind _output_get (Variables|/Game/Blueprints/Character/GlobalGameMode.GlobalGameMode_C|SetRespawnPoint (Variables|Default|GetGameMode) (Transformation|GetWorldTransform (Variables|Default|GetRespawnPoint))))
    (if (Variables|Default|GetForeverActive)
      _
      (else
        (Variables|Default|SetIsActive false)))
    (Default|SaveGame _asglobal_character (Math|Transform|MakeTransform (.location _output_get) (.rotation _output_get)))))

(event EventBeginPlay
  (bind _returnvalue (Game|GetGameMode))
  (Utilities|IsValid _returnvalue
    (:Is%20Valid
      (bind _asglobal_game_mode (Utilities|Casting|CastToGlobalGameMode _returnvalue))
      (Variables|Default|SetGameMode _asglobal_game_mode))))

(fn ConstructionScript)