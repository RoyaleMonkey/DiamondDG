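; Level-design engraving actor whose material glows brighter as the player character gets closer.
; BeginPlay creates a dynamic material instance on the first material slot of its static mesh.
; Every Tick, MakeEmissive measures the distance to player 0, clamps it between the in and out distances, and inverts it into the Emissive scalar parameter, giving a linear fade from full to none.
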(event EventBeginPlay
  (bind _returnvalue (Rendering|Material|CreateDynamicMaterialInstance (Variables|Default|GetStaticMesh) 0 0 "None" :!class /Script/Engine.PrimitiveComponent))
  (Variables|Default|SetMaterialInstance _returnvalue))

(event EventTick
  (params (DeltaSeconds :type Float%20%28single-precision%29))
  (CallFunction|MakeEmissive))

(fn ConstructionScript)

(fn MakeEmissive
  (bind _emissivedistancein (Variables|Default|GetEmissiveDistanceIn))
  (Rendering|Material|SetScalarParameterValue (Variables|Default|GetMaterialInstance) "Emissive" (Math|Float|Lerp 0.0 1.0 (- (Math|Float|MakeLiteralFloat 1.0) (/ (- (Math|Float|Clamp(Float) (Math|Vector|Distance(Vector) (Transformation|GetActorLocation (Game|GetPlayerCharacter 0)) (Transformation|GetActorLocation)) (Variables|Default|GetEmissiveDistanceIn) (Variables|Default|GetEmissiveDistanceOut)) _emissivedistancein) (- (Variables|Default|GetEmissiveDistanceOut) _emissivedistancein)))) :!class /Script/Engine.MaterialInstanceDynamic))