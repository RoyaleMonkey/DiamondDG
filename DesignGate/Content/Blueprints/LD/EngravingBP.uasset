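; Engraving level prop whose material glow varies with the player's distance while they are inside its sphere trigger.
; BeginPlay creates a dynamic material instance and sizes the trigger to MinDistance, and overlaps with the player pawn toggle IsInRange.
; While in range, Tick maps distance to AlphaLerp, driving Emissive from zero at MinDistance up to EmissiveMaxValue at MaxDistance.
; Out of range, Emissive keeps its last value.
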(event OnComponentBeginOverlap(Trigger)
  (params (OverlappedComponent :type Primitive%20Component%20Object%20Reference) (OtherActor :type Actor%20Object%20Reference) (OtherComp :type Primitive%20Component%20Object%20Reference) (OtherBodyIndex :type Integer) (bFromSweep :type Boolean) (SweepResult :type Hit%20Result%20Structure%20%28by%20ref%29))
  (if (== OtherActor (Game|Player|GetPlayerPawn 0))
    (Variables|Default|SetIsInRange true)))

(event OnComponentEndOverlap(Trigger)
  (params (OverlappedComponent :type Primitive%20Component%20Object%20Reference) (OtherActor :type Actor%20Object%20Reference) (OtherComp :type Primitive%20Component%20Object%20Reference) (OtherBodyIndex :type Integer))
  (if (== OtherActor (Game|Player|GetPlayerPawn 0))
    (Variables|Default|SetIsInRange false)))

(event EventBeginPlay
  (bind _returnvalue (Rendering|Material|CreateDynamicMaterialInstance (Rendering|Material|GetMaterial (Variables|Default|GetStaticMesh) 0) "None" "None" :!class /Script/Engine.KismetMaterialLibrary))
  (bind _output_get (Variables|Default|SetMaterialInstance _returnvalue))
  (Rendering|Material|SetMaterial (Variables|Default|GetStaticMesh) 0 _output_get)
  (Components|Sphere|SetSphereRadius (Variables|Default|GetTrigger) (Variables|Default|GetMinDistance) true))

(event EventTick
  (params (DeltaSeconds :type Float%20%28single-precision%29))
  (CallFunction|LerpEmissive)
  (if (Variables|Default|GetIsInRange)
    (Variables|Default|SetAlphaLerp (Math|Float|Max(Float) (Math|Float|NormalizetoRange (Transformation|GetDistanceTo (Game|Player|GetPlayerPawn 0) self) (Variables|Default|GetMaxDistance) (Variables|Default|GetMinDistance)) 0.0))))

(fn ConstructionScript)

(fn LerpEmissive
  (if (Variables|Default|GetIsInRange)
    (bind _output_get (Variables|Default|SetAlphaLerp (Math|Float|Min(Float) (+ 0.01 (Variables|Default|GetAlphaLerp)) 1.0)))
    (Rendering|Material|SetScalarParameterValue (Variables|Default|GetMaterialInstance) "Emissive" (Math|Float|Lerp (Variables|Default|GetEmissiveMaxValue) 0.0 _output_get) :!class /Script/Engine.MaterialInstanceDynamic)))