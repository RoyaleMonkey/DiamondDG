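; Level-design actor that repeatedly spawns an Ak (Wwise) sound at random points around itself, at random time intervals.
; Each cycle waits a random delay, then samples points within a sphere sized by the actor's X scale.
; A one-unit visibility trace rejects blocked positions, retrying until one is clear.
; The sound auto-posts at that point, then RandomSound calls itself to schedule the next.
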(event Custom|RandomSound
  (Utilities|FlowControl|Delay (Math|Random|RandomFloatinRange (Variables|Default|GetRandomDelayMin) (Variables|Default|GetRandomDelayMax)))
  (while (Variables|Default|GetSearchPosition)
    (bind _output_get (Variables|Default|SetNewPosition (+ (Transformation|GetActorLocation) (* (Math|Random|RandomUnitVector) (Math|Random|RandomFloatinRange 0.0 (* (/ (.x (Transformation|GetActorScale3D)) 2.0) 1e+02))))))
    (bind _returnvalue (Collision|LineTraceByChannel _output_get (+ _output_get "0.000000, 0,1.000000") "TraceTypeQuery1" false 0 "None"))
    (if (not _returnvalue)
      (Variables|Default|SetSearchPosition false)))
  (Class|AkGameplayStatics|SpawnAkComponentatLocation (Variables|Default|GetSound) (Variables|Default|GetNewPosition) "0, 0, 0" true)
  (Variables|Default|SetSearchPosition true)
  (CallFunction|RandomSound))

(event EventBeginPlay
  (CallFunction|RandomSound))

(fn ConstructionScript)