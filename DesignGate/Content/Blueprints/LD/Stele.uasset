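; Level stele that, once activated, grows a temporary power area where the player's music inputs trigger powers or control linked objects.
; BeginPlay spawns colored button labels for its combo, in an arc or a ring for Loop.
; Tick expands the trigger, then counts down to shutdown while lerping stele color, and blends post-process for the overlapping camera.
; Overlap binds character input: Instant combos cast shockwave, parry or slow-mo; Control levitates and outlines linked objects.
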(event OnComponentBeginOverlap(PowerTrigger)
  (params (OverlappedComponent :type Primitive%20Component%20Object%20Reference) (OtherActor :type Actor%20Object%20Reference) (OtherComp :type Primitive%20Component%20Object%20Reference) (OtherBodyIndex :type Integer) (bFromSweep :type Boolean) (SweepResult :type Hit%20Result%20Structure%20%28by%20ref%29))
  (bind _asglobal_character (Utilities|Casting|CastToGlobalCharacter OtherActor)
    (:then
      (EventDispatchers|AssignYEvent _asglobal_character (EventDispatchers|CreateEvent :!event ChangeObject))
      (switch Utilities|FlowControl|Switch|SwitchonPowerCombos (Variables|Default|GetMusicType)
        (:NewEnumerator1
          (EventDispatchers|BindEventtoOnPlayMusic _asglobal_character (delegate Custom|PowerComboInput)))
        (:NewEnumerator2
          (EventDispatchers|BindEventtoMusicPress _asglobal_character (EventDispatchers|CreateEvent :!event SendInputtoTeleObject))
          (CallFunction|LevitateandOutline true))))
    (:CastFailed
      (Utilities|Casting|CastToALS_PlayerCameraManager OtherActor)
      (Variables|Default|SetEnablePostPocess true)
      (Variables|/Script/Engine.PostProcessComponent|SetbEnabled (Variables|Default|GetPostProcess) true))))

(event OnComponentEndOverlap(PowerTrigger)
  (params (OverlappedComponent :type Primitive%20Component%20Object%20Reference) (OtherActor :type Actor%20Object%20Reference) (OtherComp :type Primitive%20Component%20Object%20Reference) (OtherBodyIndex :type Integer))
  (bind _asglobal_character (Utilities|Casting|CastToGlobalCharacter OtherActor)
    (:then
      (EventDispatchers|UnbindEventfromYEvent _asglobal_character (EventDispatchers|CreateEvent :!event ChangeObject))
      (switch Utilities|FlowControl|Switch|SwitchonPowerCombos (Variables|Default|GetMusicType)
        (:NewEnumerator1
          (EventDispatchers|UnbindEventfromOnPlayMusic _asglobal_character (delegate Custom|PowerComboInput)))
        (:NewEnumerator2
          (EventDispatchers|UnbindEventfromMusicPress _asglobal_character (EventDispatchers|CreateEvent :!event SendInputtoTeleObject))
          (CallFunction|LevitateandOutline false))))
    (:CastFailed
      (Utilities|Casting|CastToALS_PlayerCameraManager OtherActor)
      (Variables|Default|SetEnablePostPocess false))))

(event Custom|PowerComboInput
  (params (Input :type MusicInput%20Enum :default "LT"))
  (bind _success (CallFunction|Combo Input))
  (if _success
    (CallFunction|MakePower)
    (Variables|Default|SetCurrentKeyIndex 0)))

(event EventBeginPlay
  (bind _powertrigger (Variables|Default|GetPowerTrigger))
  (bind _powertrigger_2 (Variables|Default|GetPowerTrigger))
  (bind _comboinput (Variables|Default|GetComboInput))
  (bind _comboinput_2 (Variables|Default|GetComboInput))
  (bind _returnvalue (Utilities|Array|Length _comboinput_2))
  (bind (_min _max) (Components|StaticMesh|GetLocalBounds _powertrigger))
  (bind _returnvalue_2 (* _min -1.0))
  (bind _returnvalue_3 (- _returnvalue 1))
  (bind _returnvalue_4 (Math|Integer|Min(Integer) _returnvalue_3 1))
  (bind _returnvalue_5 (+ _returnvalue_2 _max))
  (bind _returnvalue_6 (/ _returnvalue_5 2.0))
  (bind _returnvalue_7 (* _returnvalue _returnvalue_4))
  (bind _returnvalue_8 (/ "100.000000,100.000000,100.000000" _returnvalue_6))
  (bind _returnvalue_9 (* _returnvalue_7 4e+01))
  (bind (_x _y _z) (Math|Vector|BreakVector _returnvalue_8))
  (|CallParentFunction)
  (Rendering|SetVisibility _powertrigger_2 false false)
  (Variables|Default|SetDefaultScale (Variables|/Script/Engine.SceneComponent|GetRelativeScale3D _powertrigger_2))
  (Transformation|SetRelativeScale3D _powertrigger_2 "0, 0, 0")
  (Variables|Default|SetExpansionCoefficient (Math|Vector|MakeVector _x (/ (* _y (.y (* (Variables|Default|GetDefaultScale) _returnvalue_5))) (.x (* (Variables|Default|GetDefaultScale) _returnvalue_5))) (/ (* _z (.z (* (Variables|Default|GetDefaultScale) _returnvalue_5))) (.x (* (Variables|Default|GetDefaultScale) _returnvalue_5)))))
  (switch Utilities|FlowControl|Switch|SwitchonPowerCombos (Variables|Default|GetMusicType)
    (:NewEnumerator1
      (for (_array_element _array_index) _comboinput_2 :!label _label
        (bind _returnvalue_10 (Game|SpawnActorfromClass "/Script/Engine.TextRenderActor" (Math|Transform|MakeTransform (+ (* (Math|Vector|GetForwardVector (Math|Rotator|MakeRotator 0.0 0.0 (+ (.yaw (Transformation|GetWorldRotation (Variables|Default|GetStele))) (+ (* (* _array_index (/ _returnvalue_9 (Math|Conversions|ToFloat(Integer) _returnvalue_3))) -1.0) (/ _returnvalue_9 2.0))))) (Math|Float|MakeLiteralFloat 6e+01)) (Transformation|GetWorldLocation (Variables|Default|GetStele)) "0,0,17.000000") (Math|Rotator|MakeRotator (.Roll (Math|Rotator|BreakRotator (Math|Rotator|MakeRotator 0.0 0.0 (+ (.yaw (Transformation|GetWorldRotation (Variables|Default|GetStele))) (+ (* (* _array_index (/ _returnvalue_9 (Math|Conversions|ToFloat(Integer) _returnvalue_3))) -1.0) (/ _returnvalue_9 2.0)))))) 9e+01 (.Yaw (Math|Rotator|BreakRotator (Math|Rotator|MakeRotator 0.0 0.0 (+ (.yaw (Transformation|GetWorldRotation (Variables|Default|GetStele))) (+ (* (* _array_index (/ _returnvalue_9 (Math|Conversions|ToFloat(Integer) _returnvalue_3))) -1.0) (/ _returnvalue_9 2.0)))))))) "Undefined" 0 0))
        (Rendering|Components|TextRender|SetHorizontalAlignment (Variables|/Script/Engine.TextRenderActor|GetTextRender _returnvalue_10) "EHTA_Center")
        (Class|TextRenderComponent|SetVerticalAlignment (Variables|/Script/Engine.TextRenderActor|GetTextRender _returnvalue_10) "EVRTA_TextCenter")
        (switch Utilities|FlowControl|Switch|SwitchonMusicInput (Utilities|Array|Get(acopy) (.valableinput _array_element))
          (:LT
            (Rendering|Components|TextRender|SetText (Variables|/Script/Engine.TextRenderActor|GetTextRender _returnvalue_10) (Utilities|Text|MakeLiteralText "LT"))
            (Rendering|Components|TextRender|SetTextRenderColor (Variables|/Script/Engine.TextRenderActor|GetTextRender _returnvalue_10) (Math|Color|MakeColor 255 0 255 255)))
          (:LB
            (Rendering|Components|TextRender|SetText (Variables|/Script/Engine.TextRenderActor|GetTextRender _returnvalue_10) (Utilities|Text|MakeLiteralText "LB"))
            (Rendering|Components|TextRender|SetTextRenderColor (Variables|/Script/Engine.TextRenderActor|GetTextRender _returnvalue_10) (Math|Color|MakeColor 255 255 0 255)))
          (:RT
            (Rendering|Components|TextRender|SetText (Variables|/Script/Engine.TextRenderActor|GetTextRender _returnvalue_10) (Utilities|Text|MakeLiteralText "RT"))
            (Rendering|Components|TextRender|SetTextRenderColor (Variables|/Script/Engine.TextRenderActor|GetTextRender _returnvalue_10) (Math|Color|MakeColor 0 255 0 255)))
          (:RB
            (Rendering|Components|TextRender|SetText (Variables|/Script/Engine.TextRenderActor|GetTextRender _returnvalue_10) (Utilities|Text|MakeLiteralText "RB"))
            (Rendering|Components|TextRender|SetTextRenderColor (Variables|/Script/Engine.TextRenderActor|GetTextRender _returnvalue_10) (Math|Color|MakeColor 0 255 255 255))))))
    (:NewEnumerator2
      (goto _label))
    (:NewEnumerator0
      (for (_array_element_2 _array_index_2) _comboinput
        (bind _returnvalue_11 (Game|SpawnActorfromClass "/Script/Engine.TextRenderActor" (Math|Transform|MakeTransform (+ (* (Math|Vector|GetForwardVector (Math|Rotator|MakeRotator 0.0 0.0 (+ (.yaw (Transformation|GetWorldRotation (Variables|Default|GetStele))) (* (* _array_index_2 (/ 3.6e+02 (Math|Conversions|ToFloat(Integer) (Utilities|Array|Length _comboinput)))) -1.0)))) (Math|Float|MakeLiteralFloat 6e+01)) (Transformation|GetWorldLocation (Variables|Default|GetStele)) "0.000000,0,17.000000") (Math|Rotator|MakeRotator (.Roll (Math|Rotator|BreakRotator (Math|Rotator|MakeRotator 0.0 0.0 (+ (.yaw (Transformation|GetWorldRotation (Variables|Default|GetStele))) (* (* _array_index_2 (/ 3.6e+02 (Math|Conversions|ToFloat(Integer) (Utilities|Array|Length _comboinput)))) -1.0))))) 9e+01 (.Yaw (Math|Rotator|BreakRotator (Math|Rotator|MakeRotator 0.0 0.0 (+ (.yaw (Transformation|GetWorldRotation (Variables|Default|GetStele))) (* (* _array_index_2 (/ 3.6e+02 (Math|Conversions|ToFloat(Integer) (Utilities|Array|Length _comboinput)))) -1.0))))))) "Undefined" 0 0))
        (if (== _array_index_2 0)
          (Transformation|SetActorScale3D _returnvalue_11 "1.500000,1.500000,1.500000"))
        (Rendering|Components|TextRender|SetHorizontalAlignment (Variables|/Script/Engine.TextRenderActor|GetTextRender _returnvalue_11) "EHTA_Center")
        (Class|TextRenderComponent|SetVerticalAlignment (Variables|/Script/Engine.TextRenderActor|GetTextRender _returnvalue_11) "EVRTA_TextCenter")
        (switch Utilities|FlowControl|Switch|SwitchonMusicInput (Utilities|Array|Get(acopy) (.valableinput _array_element_2))
          (:LT
            (Rendering|Components|TextRender|SetText (Variables|/Script/Engine.TextRenderActor|GetTextRender _returnvalue_11) (Utilities|Text|MakeLiteralText "LT"))
            (Rendering|Components|TextRender|SetTextRenderColor (Variables|/Script/Engine.TextRenderActor|GetTextRender _returnvalue_11) (Math|Color|MakeColor 255 0 255 255)))
          (:LB
            (Rendering|Components|TextRender|SetText (Variables|/Script/Engine.TextRenderActor|GetTextRender _returnvalue_11) (Utilities|Text|MakeLiteralText "LB"))
            (Rendering|Components|TextRender|SetTextRenderColor (Variables|/Script/Engine.TextRenderActor|GetTextRender _returnvalue_11) (Math|Color|MakeColor 255 255 0 255)))
          (:RT
            (Rendering|Components|TextRender|SetText (Variables|/Script/Engine.TextRenderActor|GetTextRender _returnvalue_11) (Utilities|Text|MakeLiteralText "RT"))
            (Rendering|Components|TextRender|SetTextRenderColor (Variables|/Script/Engine.TextRenderActor|GetTextRender _returnvalue_11) (Math|Color|MakeColor 0 255 0 255)))
          (:RB
            (Rendering|Components|TextRender|SetText (Variables|/Script/Engine.TextRenderActor|GetTextRender _returnvalue_11) (Utilities|Text|MakeLiteralText "RB"))
            (Rendering|Components|TextRender|SetTextRenderColor (Variables|/Script/Engine.TextRenderActor|GetTextRender _returnvalue_11) (Math|Color|MakeColor 0 255 255 255))))))))

(event EventTick
  (params (DeltaSeconds :type Float%20%28single-precision%29))
  (CallFunction|UpdatePostProcess DeltaSeconds)
  (if (Variables|Default|GetIsActive)
    (CallFunction|PowerAreaExpansion DeltaSeconds)
    (if (Math|Vector|Equal(Vector) (Variables|Default|GetDefaultScale) (Variables|/Script/Engine.SceneComponent|GetRelativeScale3D (Variables|Default|GetPowerTrigger)) 0.0001)
      (CallFunction|MakeActivationDuration DeltaSeconds))))

(fn ConstructionScript
  (|CallParentFunction))

(fn ActivateStele
  (if (not (Variables|Default|GetIsActive))
    (Variables|Default|SetIsActive true)
    (Audio|Components|Audio|Play (Variables|Default|GetSteleOn) 0.0)
    (Rendering|SetVisibility (Variables|Default|GetPowerTrigger) true false)
    (Variables|Default|SetActualActivationDuration 0.0)))

(fn PowerAreaExpansion
  (params (deltatime :type Float%20%28single-precision%29))
  (bind _expansioncoefficient (Variables|Default|GetExpansionCoefficient))
  (bind _defaultscale (Variables|Default|GetDefaultScale))
  (bind _powertrigger (Variables|Default|GetPowerTrigger))
  (bind _powertrigger_2 (Variables|Default|GetPowerTrigger))
  (bind _areapropagationspeed (Variables|Default|GetAreaPropagationSpeed))
  (bind _returnvalue (* _expansioncoefficient deltatime))
  (bind _relativescale3d (Variables|/Script/Engine.SceneComponent|GetRelativeScale3D _powertrigger_2))
  (bind _relativescale3d_2 (Variables|/Script/Engine.SceneComponent|GetRelativeScale3D _powertrigger))
  (bind _returnvalue_2 (* _returnvalue _areapropagationspeed))
  (bind _returnvalue_3 (+ _relativescale3d_2 _returnvalue_2))
  (if (Math|Boolean|ORBoolean (< (.x _relativescale3d) (.x _defaultscale)) (< (.y _relativescale3d) (.y _defaultscale)) (< (.z _relativescale3d) (.z _defaultscale)))
    (Transformation|SetRelativeScale3D (Variables|Default|GetPowerTrigger) _returnvalue_3)
    (bind _returnvalue_4 (Rendering|Material|CreateDynamicMaterialInstance (Variables|Default|GetStaticMesh) 0 0 "None" :!class /Script/Engine.PrimitiveComponent))
    (Rendering|Material|SetVectorParameterValue _returnvalue_4 "Color" (Math|Color|Lerp(LinearColor) (Variables|Default|GetColorOff) (Variables|Default|GetColorOn) (/ (Math|Vector|VectorLengthSquared _returnvalue_3) (Math|Vector|VectorLengthSquared (Variables|Default|GetDefaultScale)))) :!class /Script/Engine.MaterialInstanceDynamic)
    (else
      (Transformation|SetRelativeScale3D (Variables|Default|GetPowerTrigger) (Variables|Default|GetDefaultScale))
      (bind _returnvalue_5 (Rendering|Material|CreateDynamicMaterialInstance (Variables|Default|GetStaticMesh) 0 0 "None" :!class /Script/Engine.PrimitiveComponent))
      (Rendering|Material|SetVectorParameterValue _returnvalue_5 "Color" (Variables|Default|GetColorOn) :!class /Script/Engine.MaterialInstanceDynamic))))

(fn MakeActivationDuration
  (params (deltaTime :type Float%20%28single-precision%29))
  (bind _powertrigger (Variables|Default|GetPowerTrigger))
  (bind _activationduration (Variables|Default|GetActivationDuration))
  (if (>= (+ (Variables|Default|GetActualActivationDuration) deltaTime) _activationduration)
    (Variables|Default|SetActualActivationDuration _activationduration)
    (bind _returnvalue (Rendering|Material|CreateDynamicMaterialInstance (Variables|Default|GetStaticMesh) 0 0 "None" :!class /Script/Engine.PrimitiveComponent))
    (Rendering|Material|SetVectorParameterValue _returnvalue "Color" (Variables|Default|GetColorOff) :!class /Script/Engine.MaterialInstanceDynamic)
    (Variables|Default|SetIsActive false)
    (Rendering|SetVisibility _powertrigger false false)
    (Transformation|SetRelativeScale3D _powertrigger "0, 0, 0")
    (else
      (bind _output_get (Variables|Default|SetActualActivationDuration (+ (Variables|Default|GetActualActivationDuration) deltaTime)))
      (bind _returnvalue_2 (Rendering|Material|CreateDynamicMaterialInstance (Variables|Default|GetStaticMesh) 0 0 "None" :!class /Script/Engine.PrimitiveComponent))
      (Rendering|Material|SetVectorParameterValue _returnvalue_2 "Color" (Math|Color|Lerp(LinearColor) (Variables|Default|GetColorOn) (Variables|Default|GetColorOff) (/ _output_get _activationduration)) :!class /Script/Engine.MaterialInstanceDynamic))))

(fn InstantInteract
  (CallFunction|ActivateStele))

(fn MakePower
  (bind _character (Variables|Default|GetCharacter))
  (switch Utilities|FlowControl|Switch|SwitchonPowerEnum (Variables|Default|GetareaType)
    (:NewEnumerator5
      (Default|TrytoMakeShockWave _character))
    (:NewEnumerator9
      (Default|TrytoParry _character))
    (:NewEnumerator10
      (Default|LaunchSlowSphere (Variables|/Game/Blueprints/Character/GlobalCharacter.GlobalCharacter_C|GetSlowMoComponent _character)))))

(fn LoopStart
  (CallFunction|ActivateStele))

(fn SendInputtoTeleObject
  (params (Press%20? :type Boolean) (NewParam1 :type MusicInput%20Enum :default "LT"))
  (Default|Listen (Utilities|Array|Get(acopy) (Variables|Default|GetLinkedObjects) (Variables|Default|GetLinkedObjectIndex)) NewParam1 Press%20?))

(fn UpdatePostProcess
  (params (DeltaSeconds :type Float%20%28single-precision%29))
  (bind _postpocesstransitionduration (Variables|Default|GetPostPocessTransitionDuration))
  (bind _postprocess (Variables|Default|GetPostProcess))
  (if (Variables|Default|GetEnablePostPocess)
    (bind _output_get (Variables|Default|SetActualPostPocessTransitionDuration (Math|Float|Min(Float) (+ (Variables|Default|GetActualPostPocessTransitionDuration) DeltaSeconds) _postpocesstransitionduration)))
    (Variables|/Script/Engine.PostProcessComponent|SetBlendWeight _postprocess (/ _output_get _postpocesstransitionduration))
    (else
      (bind _output_get_2 (Variables|Default|SetActualPostPocessTransitionDuration (Math|Float|Max(Float) (- (Variables|Default|GetActualPostPocessTransitionDuration) DeltaSeconds) 0.0)))
      (bind _output_get_3 (Variables|/Script/Engine.PostProcessComponent|SetBlendWeight _postprocess (/ _output_get_2 (Variables|Default|GetPostPocessTransitionDuration))))
      (if (== _output_get_3 0.0)
        (Variables|/Script/Engine.PostProcessComponent|SetbEnabled (Variables|Default|GetPostProcess) false)))))

(fn ChangeObject
  (CallFunction|LevitateandOutline false)
  (bind _result (Math|Integer|IncrementInt (Variables|Default|GetLinkedObjectIndex))
    (:%20%20
      (if (<= (Utilities|Array|Length (Variables|Default|GetLinkedObjects)) _result)
        (Variables|Default|SetLinkedObjectIndex 0))
      (CallFunction|LevitateandOutline true))))

(fn LevitateandOutline
  (params (active :type Boolean))
  (bind _linkedobjects (Variables|Default|GetLinkedObjects))
  (bind _linkedobjectindex (Variables|Default|GetLinkedObjectIndex))
  (bind _linkedobjects_2 (Variables|Default|GetLinkedObjects))
  (bind _linkedobjectindex_2 (Variables|Default|GetLinkedObjectIndex))
  (bind _output (Utilities|Array|Get(acopy) _linkedobjects _linkedobjectindex))
  (bind _output_2 (Utilities|Array|Get(acopy) _linkedobjects_2 _linkedobjectindex_2))
  (if active
    (Default|Levitate _output_2)
    (Default|SetOutlineVisibility _output_2 true)
    (else
      (Default|StopLevitate _output)
      (Default|SetOutlineVisibility _output false))))