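; A level-design statue that glows while the telekinetic area linked to its TelekineticObject is moving.
; BeginPlay swaps the static mesh's first material for a dynamic instance.
; Each tick, if that area is valid, one alpha ramps up while it moves and down while it is still, clamped between 0 and 1, driving the Emissive parameter for a roughly one-second fade each way.
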(event EventTick
  (params (DeltaSeconds :type Float%20%28single-precision%29))
  (if (Utilities|IsValid (Variables|/Game/Blueprints/LD/TelekineticBPs/TelekineticObjectComponent.TelekineticObjectComponent_C|GetTelekineticArea (Variables|Default|GetTelekineticObject)))
    (CallFunction|LerpEmissiveUp DeltaSeconds)
    (CallFunction|LerpEmissiveDown DeltaSeconds)))

(event EventBeginPlay
  (bind _returnvalue (Rendering|Material|CreateDynamicMaterialInstance (Rendering|Material|GetMaterial (Variables|Debug|GetStaticMeshComponent) 0) "None" "None" :!class /Script/Engine.KismetMaterialLibrary))
  (bind _output_get (Variables|Default|SetMaterialInstance _returnvalue))
  (Rendering|Material|SetMaterial (Variables|Debug|GetStaticMeshComponent) 0 _output_get))

(fn ConstructionScript)

(fn LerpEmissiveUp
  (params (Tick :type Float%20%28single-precision%29))
  (if (Variables|/Game/Blueprints/LD/TelekineticBPs/TelekineticArea.TelekineticArea_C|GetisMoving? (Variables|/Game/Blueprints/LD/TelekineticBPs/TelekineticObjectComponent.TelekineticObjectComponent_C|GetTelekineticArea (Variables|Default|GetTelekineticObject)))
    (bind _output_get (Variables|Default|SetAlphaLerp (Math|Float|Min(Float) (+ Tick (Variables|Default|GetAlphaLerp)) 1.0)))
    (Rendering|Material|SetScalarParameterValue (Variables|Default|GetMaterialInstance) "Emissive" (Math|Float|Lerp 0.0 1.0 _output_get) :!class /Script/Engine.MaterialInstanceDynamic)))

(fn LerpEmissiveDown
  (params (Tick :type Float%20%28single-precision%29))
  (if (not (Variables|/Game/Blueprints/LD/TelekineticBPs/TelekineticArea.TelekineticArea_C|GetisMoving? (Variables|/Game/Blueprints/LD/TelekineticBPs/TelekineticObjectComponent.TelekineticObjectComponent_C|GetTelekineticArea (Variables|Default|GetTelekineticObject))))
    (bind _output_get (Variables|Default|SetAlphaLerp (Math|Float|Max(Float) (- (Variables|Default|GetAlphaLerp) Tick) 0.0)))
    (Rendering|Material|SetScalarParameterValue (Variables|Default|GetMaterialInstance) "Emissive" (Math|Float|Lerp 0.0 1.0 _output_get) :!class /Script/Engine.MaterialInstanceDynamic)))