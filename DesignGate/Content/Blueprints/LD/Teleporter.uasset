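; Level-design teleporter actor that sends an overlapping GlobalCharacter to the place chosen by its Destination enum.
; On BeginPlay, that enum sets the text label and the Plane's preview material, with most destinations sharing a test-scene material.
; On overlap, HUB, Art and Features open levels, while ability areas move the character to ArrivalPoint.
; Sand Box has no overlap action, and Tuto opens a level named "None".
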(event EventBeginPlay
  (bind _textrender (Variables|Default|GetTextRender))
  (bind _plane (Variables|Default|GetPlane))
  (switch Utilities|FlowControl|Switch|SwitchonTeleportDestEnum (Variables|Default|GetDestination)
    (:NewEnumerator0
      (Rendering|Components|TextRender|SetText _textrender (Utilities|Text|MakeLiteralText "HUB"))
      (Rendering|Material|SetMaterial _plane 0 "/Game/Assets/GPAssets/Material/HUBPreview_Mat.HUBPreview_Mat"))
    (:NewEnumerator1
      (Rendering|Components|TextRender|SetText _textrender (Utilities|Text|MakeLiteralText "Art Scene"))
      (Rendering|Material|SetMaterial _plane 0 "/Game/Assets/GPAssets/Material/ArtScenePreview_Mat.ArtScenePreview_Mat"))
    (:NewEnumerator2
      (Rendering|Components|TextRender|SetText _textrender (Utilities|Text|MakeLiteralText "Features Scene"))
      (Rendering|Material|SetMaterial _plane 0 "/Game/Assets/GPAssets/Material/TestScenePreview_Mat.TestScenePreview_Mat" :!label _label))
    (:NewEnumerator3
      (Rendering|Components|TextRender|SetText _textrender (Utilities|Text|MakeLiteralText "Sandbox"))
      (goto _label))
    (:NewEnumerator4
      (Rendering|Components|TextRender|SetText _textrender (Utilities|Text|MakeLiteralText "GliderTower"))
      (goto _label))
    (:NewEnumerator5
      (Rendering|Components|TextRender|SetText _textrender (Utilities|Text|MakeLiteralText "Geyser"))
      (Rendering|Material|SetMaterial _plane 0 "/Game/Assets/GPAssets/Material/TestScenePreview_Mat.TestScenePreview_Mat"))
    (:NewEnumerator6
      (Rendering|Components|TextRender|SetText _textrender (Utilities|Text|MakeLiteralText "Dash"))
      (Rendering|Material|SetMaterial _plane 0 "/Game/Assets/GPAssets/Material/TestScenePreview_Mat.TestScenePreview_Mat"))
    (:NewEnumerator7
      (Rendering|Components|TextRender|SetText _textrender (Utilities|Text|MakeLiteralText "Squall"))
      (Rendering|Material|SetMaterial _plane 0 "/Game/Assets/GPAssets/Material/TestScenePreview_Mat.TestScenePreview_Mat"))
    (:NewEnumerator8
      (Rendering|Components|TextRender|SetText _textrender (Utilities|Text|MakeLiteralText "Shockwave"))
      (Rendering|Material|SetMaterial _plane 0 "/Game/Assets/GPAssets/Material/TestScenePreview_Mat.TestScenePreview_Mat"))
    (:NewEnumerator9
      (Rendering|Components|TextRender|SetText _textrender (Utilities|Text|MakeLiteralText "Tuto"))
      (Rendering|Material|SetMaterial _plane 0 "/Game/Assets/GPAssets/Material/TestScenePreview_Mat.TestScenePreview_Mat"))))

(event Collision|EventActorBeginOverlap
  (params (OtherActor :type Actor%20Object%20Reference))
  (bind _asglobal_character (Utilities|Casting|CastToGlobalCharacter OtherActor))
  (switch Utilities|FlowControl|Switch|SwitchonTeleportDestEnum (Variables|Default|GetDestination)
    (:NewEnumerator0
      (Game|OpenLevel(byName) "HubScene"))
    (:NewEnumerator1
      (Game|OpenLevel(byName) "Yoan"))
    (:NewEnumerator2
      (Game|OpenLevel(byName) "GlobalTestScene"))
    (:NewEnumerator4
      (Transformation|SetActorRelativeLocation _asglobal_character (Transformation|GetWorldLocation (Variables|Default|GetarrivalPoint)) :!label _label))
    (:NewEnumerator5
      (goto _label))
    (:NewEnumerator6
      (goto _label))
    (:NewEnumerator7
      (goto _label))
    (:NewEnumerator8
      (goto _label))
    (:NewEnumerator9
      (Game|OpenLevel(byName) "None"))))

(event EventTick
  (params (DeltaSeconds :type Float%20%28single-precision%29)))

(fn ConstructionScript)