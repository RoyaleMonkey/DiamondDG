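; Level-design turret Blueprint that periodically fires SphereShieldCollision actors as its projectiles.
; Tick accumulates delta time and calls the Shoot event whenever the elapsed time reaches SpawnDelay, then resets the timer.
; Shoot spawns the projectile at the ShotPosition component's world location with zero rotation, ignoring the turret's orientation, and sets its LifeTime from BulletLifeTime.
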(event Custom|Shoot
  (bind _returnvalue (Game|SpawnActorfromClass "/Game/Blueprints/Others/SphereShieldCollision.SphereShieldCollision_C" (Math|Transform|MakeTransform (Transformation|GetWorldLocation (Variables|Default|GetShotPosition))) "Undefined" 0 0))
  (Variables|/Game/Blueprints/Others/SphereShieldCollision.SphereShieldCollision_C|SetLifeTime _returnvalue (Variables|Default|GetBulletLifeTime)))

(event EventTick
  (params (DeltaSeconds :type Float%20%28single-precision%29))
  (if (>= (Variables|Default|GetActualSpawnDelay) (Variables|Default|GetSpawnDelay))
    (Variables|Default|SetActualSpawnDelay 0.0)
    (CallFunction|Shoot)
    (else
      (Variables|Default|SetActualSpawnDelay (+ (Variables|Default|GetActualSpawnDelay) DeltaSeconds)))))

(fn ConstructionScript)