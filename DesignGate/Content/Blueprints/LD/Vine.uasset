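; Level-design vine actor that builds a deformable mesh along an editable spline, with no runtime logic.
; The construction script adds one spline mesh component per segment between neighboring spline points, matching their local positions and tangents.
; Each point's Y and Z scale sets the segment's cross-section, so thickness can vary along the vine.
; Roll-matching nodes exist but are disconnected, so point roll is not applied.
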(event EventBeginPlay)

(event Collision|EventActorBeginOverlap
  (params (OtherActor :type Actor%20Object%20Reference)))

(event EventTick
  (params (DeltaSeconds :type Float%20%28single-precision%29)))

(fn ConstructionScript
  (bind _spline (Variables|Default|GetSpline))
  (for _index (range 0 (- (Spline|GetNumberOfSplinePoints _spline) 2))
    (bind _returnvalue (AddComponent|AddSplineMeshComponent false))
    (Transformation|AttachComponentToComponent _returnvalue (Variables|Default|GetDefaultSceneRoot) "None" "KeepWorld" "KeepWorld" "KeepWorld" true)
    (SplineMesh|SetStartandEnd _returnvalue (.Location (Spline|GetLocationandTangentatSplinePoint _spline _index "Local")) (.Tangent (Spline|GetLocationandTangentatSplinePoint _spline _index "Local")) (.Location (Spline|GetLocationandTangentatSplinePoint _spline (+ _index 1) "Local")) (.Tangent (Spline|GetLocationandTangentatSplinePoint _spline (+ _index 1) "Local")) false :!class /Script/Engine.SplineMeshComponent)
    (SplineMesh|SetStartScale _returnvalue (Math|Vector2D|MakeVector2D (.y (Spline|GetScaleatSplinePoint _spline _index)) (.z (Spline|GetScaleatSplinePoint _spline _index))) false :!class /Script/Engine.SplineMeshComponent)
    (SplineMesh|SetEndScale _returnvalue (Math|Vector2D|MakeVector2D (.y (Spline|GetScaleatSplinePoint _spline (+ _index 1))) (.z (Spline|GetScaleatSplinePoint _spline (+ _index 1)))) true :!class /Script/Engine.SplineMeshComponent)))