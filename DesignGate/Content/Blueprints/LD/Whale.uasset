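; Level-design whale actor that swims once along a spline when a GlobalCharacter first enters its activation trigger.
; The construction script places the whale at the spline start, and Tick advances it by distance at a set speed, matching spline rotation, until it reaches the end.
; Past a set fraction of the path it fires the water-jet Niagara effect and Wwise blow sound, then raises that threshold out of reach so they play once.
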(event OnComponentBeginOverlap(ActivationTrigger)
  (params (OverlappedComponent :type Primitive%20Component%20Object%20Reference) (OtherActor :type Actor%20Object%20Reference) (OtherComp :type Primitive%20Component%20Object%20Reference) (OtherBodyIndex :type Integer) (bFromSweep :type Boolean) (SweepResult :type Hit%20Result%20Structure%20%28by%20ref%29))
  (Utilities|Casting|CastToGlobalCharacter OtherActor)
  (if (not (Variables|Default|GetIsActivated))
    (Variables|Default|SetIsActivated true)
    (Variables|Default|SetMoveWhale true)))

(event EventTick
  (params (DeltaSeconds :type Float%20%28single-precision%29))
  (Utilities|FlowControl|Sequence
    (:then_0
      (CallFunction|MoveWhaleonTrajectory DeltaSeconds))))

(fn ConstructionScript
  (bind _trajectory (Variables|Default|GetTrajectory))
  (Transformation|SetWorldLocationAndRotation (Variables|Default|GetWhale) (Spline|GetLocationatDistanceAlongSpline _trajectory 0.0 "World") (Spline|GetRotationatDistanceAlongSpline _trajectory 0.0 "World") false false))

(fn MoveWhaleonTrajectory
  (params (DeltaSeconds :type Float%20%28single-precision%29))
  (bind _trajectory (Variables|Default|GetTrajectory))
  (bind _trajectory_2 (Variables|Default|GetTrajectory))
  (bind _returnvalue (Spline|GetSplineLength _trajectory_2))
  (if (Variables|Default|GetMoveWhale)
    (bind _output_get (Variables|Default|SetCurrentPositionOnTrajectory (Utilities|IncrementFloat (Variables|Default|GetCurrentPositionOnTrajectory) (* DeltaSeconds (Variables|Default|GetSpeed) 1e+02) _returnvalue)))
    (Utilities|FlowControl|Sequence
      (:then_0
        (Transformation|SetWorldLocationAndRotation (Variables|Default|GetWhale) (Spline|GetLocationatDistanceAlongSpline _trajectory _output_get "World") (Spline|GetRotationatDistanceAlongSpline _trajectory _output_get "World") false false)
        (if (== (Variables|Default|GetCurrentPositionOnTrajectory) (Spline|GetSplineLength (Variables|Default|GetTrajectory)))
          (Variables|Default|SetMoveWhale false)))
      (:then_1
        (if (> (/ (Variables|Default|GetCurrentPositionOnTrajectory) _returnvalue) (Variables|Default|GetWhaleJetRatio))
          (Components|Activation|Activate (Variables|Default|GetNS_whale) true)
          (Class|AkGameplayStatics|PostEvent "/Game/Audio/Events/LE/SFX_Whale/Play_SFX_LE_Whale_Water_Blow.Play_SFX_LE_Whale_Water_Blow" self)
          (Variables|Default|SetWhaleJetRatio 2.0))))))