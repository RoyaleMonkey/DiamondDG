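; SphereShieldCollision is an actor that moves in a straight line for a limited lifetime, named as a collision body for a sphere shield.
; Each Tick offsets its location by Force scaled by delta time, using a swept move so blocking collision is respected.
; Force acts as a velocity here, and the actor destroys itself once its accumulated ActualLifeTime reaches LifeTime.
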(event EventTick
  (params (DeltaSeconds :type Float%20%28single-precision%29))
  (Transformation|SetActorLocation (+ (Transformation|GetActorLocation) (* (Variables|Default|Getforce) DeltaSeconds)) true false)
  (bind _output_get (Variables|Default|SetActualLifeTime (+ (Variables|Default|GetActualLifeTime) DeltaSeconds)))
  (if (>= _output_get (Variables|Default|GetLifeTime))
    (Actor|DestroyActor)))

(fn ConstructionScript)