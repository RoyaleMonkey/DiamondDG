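; GhostBP is a ghost actor that resizes itself to represent either a Cube or a Wall.
; The construction script caches the first valid top-level GlobalTestWidget it finds.
; ChangeGhostType sets actor scale from that widget's values: per-axis scale for a Cube, or thickness and width with a fixed height for a Wall.
; The event graph holds no active logic, so scale updates only when that function is called.
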(event EventBeginPlay)

(event Collision|EventActorBeginOverlap
  (params (OtherActor :type Actor%20Object%20Reference)))

(event EventTick
  (params (DeltaSeconds :type Float%20%28single-precision%29)))

(fn ConstructionScript
  ;[1 1 1] Get Widget
  (bind _foundwidgets (Widget|GetAllWidgetsOfClass "/Game/Assets/GPAssets/Widget/GlobalTestWidget.GlobalTestWidget_C" true))
  (Utilities|IsValid (Utilities|Array|Get(acopy) _foundwidgets)
    (:Is%20Valid
      (Variables|Default|SetFound%20Widgets (Utilities|Array|Get(acopy) _foundwidgets)))))

(fn ChangeGhostType
  (params (newType :type GhostTypeEnum%20Enum :default "NewEnumerator0"))
  (bind _found_widgets (Variables|Default|GetFound%20Widgets))
  (switch Utilities|FlowControl|Switch|SwitchonGhostTypeEnum newType
    (:NewEnumerator0
      (Transformation|SetActorScale3D (Math|Vector|MakeVector (Class|SpinBox|GetValue (Variables|/Game/Assets/GPAssets/Widget/GlobalTestWidget.GlobalTestWidget_C|GetCubeScaleX _found_widgets)) (Class|SpinBox|GetValue (Variables|/Game/Assets/GPAssets/Widget/GlobalTestWidget.GlobalTestWidget_C|GetCubeScaleY _found_widgets)) (Class|SpinBox|GetValue (Variables|/Game/Assets/GPAssets/Widget/GlobalTestWidget.GlobalTestWidget_C|GetCubeScaleZ _found_widgets)))))
    (:NewEnumerator1
      ;[1 1 1] Set width
      (Transformation|SetActorScale3D (Math|Vector|MakeVector (Class|SpinBox|GetValue (Variables|/Game/Assets/GPAssets/Widget/GlobalTestWidget.GlobalTestWidget_C|GetWallThickness (Variables|Default|GetFound%20Widgets))) (Class|SpinBox|GetValue (Variables|/Game/Assets/GPAssets/Widget/GlobalTestWidget.GlobalTestWidget_C|GetWallWidth (Variables|Default|GetFound%20Widgets))) 5.0)))))