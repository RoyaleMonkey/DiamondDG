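; Spawnable wall actor that rises into place after a delay, then destroys itself after a set duration unless that duration is -1.
; The construction script reads offset, size and timings from the first GlobalTestWidget found, so a live test UI tunes each spawn.
; Tick lerps the wall mesh's relative Z up from StartZ.
; SpawnWithGroundLocation clears the forward offset and raises the start position for ground-targeted placement.
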(event EventBeginPlay
  (bind _duration (Variables|Default|GetDuration))
  (Utilities|FlowControl|Sequence
    (:then_0
      (Utilities|FlowControl|Delay (Variables|Default|GetriseDelay))
      (Variables|Default|SetIsRising true)
      (if (!= _duration -1.0)
        (Utilities|FlowControl|Delay _duration)
        (Actor|DestroyActor)))
    (:then_1
      (Rendering|SetActorHiddenInGame false))))

(event EventTick
  (params (DeltaSeconds :type Float%20%28single-precision%29))
  (if (Variables|Default|GetIsRising)
    ;[1 1 1] Rise Update
    (bind _output_get (Variables|Default|Settimer (+ (Variables|Default|Gettimer) DeltaSeconds)))
    (Transformation|SetRelativeLocation (Variables|Default|GetWall) (+ (Variables|Default|GetStartLocation) (Math|Vector|MakeVector 0.0 0.0 (Math|Float|Lerp (Variables|Default|GetStartZ) 0.0 (/ _output_get (Variables|Default|GetRiseDuration))))) false false)
    (if (> (Variables|Default|Gettimer) (Variables|Default|GetRiseDuration))
      (Variables|Default|SetIsRising false))))

(fn ConstructionScript
  ;[1 1 1] Get Widget
  (bind _foundwidgets (Widget|GetAllWidgetsOfClass "/Game/Assets/GPAssets/Widget/GlobalTestWidget.GlobalTestWidget_C" true))
  (Utilities|IsValid (Utilities|Array|Get(acopy) _foundwidgets)
    (:Is%20Valid
      (Variables|Default|SetFound%20Widgets (Utilities|Array|Get(acopy) _foundwidgets))
      (Utilities|FlowControl|Sequence
        (:then_0
          ;[1 1 1] Set Offset
          (bind _output_get (Variables|Default|SetStartLocation (Math|Vector|MakeVector (Class|SpinBox|GetValue (Variables|/Game/Assets/GPAssets/Widget/GlobalTestWidget.GlobalTestWidget_C|GetWallOffset (Variables|Default|GetFound%20Widgets))) 0.0 0.0)))
          (Transformation|SetRelativeLocation (Variables|Default|GetWall) (+ _output_get (Math|Vector|MakeVector 0.0 0.0 (Variables|Default|GetStartZ))) false false)
          (Rendering|SetActorHiddenInGame true))
        (:then_1
          ;[1 1 1] Set width
          (Transformation|SetRelativeScale3D (Variables|Default|GetWall) (Math|Vector|MakeVector (Class|SpinBox|GetValue (Variables|/Game/Assets/GPAssets/Widget/GlobalTestWidget.GlobalTestWidget_C|GetWallThickness (Variables|Default|GetFound%20Widgets))) (Class|SpinBox|GetValue (Variables|/Game/Assets/GPAssets/Widget/GlobalTestWidget.GlobalTestWidget_C|GetWallWidth (Variables|Default|GetFound%20Widgets))) 3.0)))
        (:then_2
          ;[1 1 1] Set rise Duration
          (Variables|Default|SetRiseDuration (Class|SpinBox|GetValue (Variables|/Game/Assets/GPAssets/Widget/GlobalTestWidget.GlobalTestWidget_C|GetWallRiseDuration (Variables|Default|GetFound%20Widgets)))))
        (:then_3
          ;[1 1 1] Set Duration
          (Variables|Default|SetDuration (Class|SpinBox|GetValue (Variables|/Game/Assets/GPAssets/Widget/GlobalTestWidget.GlobalTestWidget_C|GetWallDuration (Variables|Default|GetFound%20Widgets)))))
        (:then_4
          ;[1 1 1] Rise Delay
          (Variables|Default|SetriseDelay (Class|SpinBox|GetValue (Variables|/Game/Assets/GPAssets/Widget/GlobalTestWidget.GlobalTestWidget_C|GetWallRiseDelay (Variables|Default|GetFound%20Widgets)))))))))

(fn SpawnwithGroundLocation
  (bind _output_get (Variables|Default|SetStartLocation (+ (Variables|Default|GetStartLocation) (Math|Vector|MakeVector (* -1 (.x (Variables|Default|GetStartLocation))) 0.0 1e+02))))
  (Transformation|SetRelativeLocation (Variables|Default|GetWall) (+ _output_get (Math|Vector|MakeVector 0.0 0.0 (Variables|Default|GetStartZ))) false false))