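; LoopComponent is a rhythm-combo component for GlobalCharacter that judges key inputs against a repeating tempo to activate the character's current stele.
; While Activated, Tick advances the beat timer and fires force feedback slightly before each beat.
; InputReceived accepts presses within a margin around the beat, toggles an inactive stele once the index passes the combo's length, and rejects off-beat presses with a sound.
; Tick also breaks the combo when a beat gets no input.
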(event EventBeginPlay
  (bind _asglobal_character (Utilities|Casting|CastToGlobalCharacter (Components|GetOwner)))
  (Variables|Default|SetGlobal%20Character _asglobal_character))

(event EventTick
  (params (DeltaSeconds :type Float%20%28single-precision%29))
  (Utilities|FlowControl|Sequence
    (:then_0
      ;[1 1 1] TempoVibration
      (if (Variables|Default|GetActivated)
        (bind _output_get (Variables|Default|SetTempoTimer (+ (Variables|Default|GetTempoTimer) DeltaSeconds)))
        (if (> _output_get (- (Variables|Default|GetTempo) (Variables|Default|GetVibrationOffset)))
          (if (not (Variables|Default|GetVibrationActivated))
            (Game|Feedback|ClientPlayForceFeedback (Game|GetPlayerController 0) "/Game/Blueprints/CustomParam/TempoVibration.TempoVibration" "None" false false false)
            (Variables|Default|SetVibrationActivated true)
            (elif (> (Variables|Default|GetTempoTimer) (Variables|Default|GetTempo))
              (Variables|Default|SetTempoTimer 0.0)
              (Variables|Default|SetVibrationActivated false))))))
    (:then_1
      ;[1 1 1] StopCombo if no key
      (if (Math|Boolean|ANDBoolean (Variables|Default|GetComboStart) (not (Variables|Default|GetComboValidate)) (> (Variables|Default|GetTempoTimer) (Variables|Default|GetMargin)) (< (Variables|Default|GetTempoTimer) (- (Variables|Default|GetTempo) (Variables|Default|GetMargin))))
        (if (not (Variables|Default|GetComboContinue))
          (Variables|Default|SetComboStart false)
          (Variables|/Game/Blueprints/Character/GlobalCharacter.GlobalCharacter_C|SetCurrentKeyIndex (Variables|Default|GetGlobal%20Character) 0)
          (Audio|PlaySound2D "/Game/Sounds/Sounds/WrongKey.WrongKey" 1.0 1.0 0.0 0 0)
          (else
            (Variables|Default|SetComboValidate true)
            (Variables|Default|SetComboContinue false)))))
    (:then_2
      (if (and (> (Variables|Default|GetTempoTimer) (- (Variables|Default|GetTempo) (Variables|Default|GetMargin))) (Variables|Default|GetComboValidate))
        (Variables|Default|SetComboValidate false)))))

(fn InputReceived
  (params (Index :type Integer%20%28by%20ref%29))
  (bind _global_character (Variables|Default|GetGlobal%20Character))
  (bind _currentstele (Variables|/Game/Blueprints/Character/GlobalCharacter.GlobalCharacter_C|GetCurrentStele _global_character))
  (if (or (> (Variables|Default|GetTempoTimer) (- (Variables|Default|GetTempo) (Variables|Default|GetMargin))) (< (Variables|Default|GetTempoTimer) (Variables|Default|GetMargin)))
    (Variables|Default|SetComboStart true)
    (Variables|Default|SetComboContinue true)
    (if (>= Index (Utilities|Array|Length (Variables|/Game/Blueprints/Character/GlobalCharacter.GlobalCharacter_C|GetComboKeys (Variables|Default|GetGlobal%20Character))))
      (|SetBy-RefVar Index)
      (if (not (Variables|/Game/Blueprints/PowerAreaBP/Stele.Stele_C|GetIsActive _currentstele))
        (Default|ToggleActivation _currentstele)))
    (else
      (Audio|PlaySound2D "/Game/Sounds/Sounds/WrongKey.WrongKey" 1.0 1.0 0.0 0 0)
      (Variables|Default|SetComboStart false)
      (|SetBy-RefVar Index))))