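; SpawnableWall is a wall actor that rises from below after a delay and can destroy itself after a set lifetime.
; Its construction script reads offset, thickness, width, rise time, delay and lifetime from text fields in the first TestPowerArea widget found.
; Tick lerps the Wall component's relative height up to zero over the rise time.
; The lifetime counts from the rise start, and -1 keeps the wall indefinitely.
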(event EventBeginPlay
  (bind _duration (Variables|Default|GetDuration))
  (Utilities|FlowControl|Sequence
    (:then_0
      (Utilities|FlowControl|Delay (Variables|Default|GetriseDelay))
      (Variables|Default|SetIsRising true)
      (if (!= _duration -1.0)
        (Utilities|FlowControl|Delay _duration)
        (Actor|DestroyActor)))))

(event EventTick
  (params (DeltaSeconds :type Float%20%28single-precision%29))
  (if (Variables|Default|GetIsRising)
    ;[1 1 1] Rise Update
    (bind _output_get (Variables|Default|Settimer (+ (Variables|Default|Gettimer) DeltaSeconds)))
    (Transformation|SetRelativeLocation (Variables|Default|GetWall) (+ (Variables|Default|GetStartLocation) (Math|Vector|MakeVector 0.0 0.0 (Math|Float|Lerp -2.3e+02 0.0 (/ _output_get (Variables|Default|GetRiseDuration))))) false false)
    (if (> (Variables|Default|Gettimer) (Variables|Default|GetRiseDuration))
      (Variables|Default|SetIsRising false))))

(fn ConstructionScript
  ;[1 1 1] Get Widget
  (bind _foundwidgets (Widget|GetAllWidgetsOfClass "/Game/Assets/GPAssets/Widget/TestPowerArea.TestPowerArea_C" true))
  (Utilities|IsValid (Utilities|Array|Get(acopy) _foundwidgets)
    (:Is%20Valid
      (Variables|Default|SetFound%20Widgets (Utilities|Array|Get(acopy) _foundwidgets))
      (Utilities|FlowControl|Sequence
        (:then_0
          ;[1 1 1] Set Offset
          (Variables|Default|SetStartLocation (Math|Vector|MakeVector (Math|Conversions|ToFloat(Integer) (Utilities|String|ToString(Text) (Class|EditableTextBox|GetText (Variables|/Game/Assets/GPAssets/Widget/TestPowerArea.TestPowerArea_C|Getoffset (Variables|Default|GetFound%20Widgets))))) 0.0 0.0)))
        (:then_1
          ;[1 1 1] Set width
          (Transformation|SetRelativeScale3D (Variables|Default|GetWall) (Math|Vector|MakeVector (Math|Conversions|ToFloat(Integer) (Utilities|String|ToString(Text) (Class|EditableTextBox|GetText (Variables|/Game/Assets/GPAssets/Widget/TestPowerArea.TestPowerArea_C|Getthick (Variables|Default|GetFound%20Widgets))))) (Math|Conversions|ToFloat(Integer) (Utilities|String|ToString(Text) (Class|EditableTextBox|GetText (Variables|/Game/Assets/GPAssets/Widget/TestPowerArea.TestPowerArea_C|Getwidth (Variables|Default|GetFound%20Widgets))))) 3.0)))
        (:then_2
          ;[1 1 1] Set rise Duration
          (Variables|Default|SetRiseDuration (Math|Conversions|ToFloat(Integer) (Utilities|String|ToString(Text) (Class|EditableTextBox|GetText (Variables|/Game/Assets/GPAssets/Widget/TestPowerArea.TestPowerArea_C|GetriseDuration (Variables|Default|GetFound%20Widgets)))))))
        (:then_3
          ;[1 1 1] Set Duration
          (Variables|Default|SetDuration (Math|Conversions|ToFloat(Integer) (Utilities|String|ToString(Text) (Class|EditableTextBox|GetText (Variables|/Game/Assets/GPAssets/Widget/TestPowerArea.TestPowerArea_C|Getduration (Variables|Default|GetFound%20Widgets)))))))
        (:then_4
          ;[1 1 1] Rise Delay
          (Variables|Default|SetriseDelay (Math|Conversions|ToFloat(Integer) (Utilities|String|ToString(Text) (Class|EditableTextBox|GetText (Variables|/Game/Assets/GPAssets/Widget/TestPowerArea.TestPowerArea_C|Getdelay (Variables|Default|GetFound%20Widgets)))))))))))