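; Stele actor that grants a timed power area to GlobalCharacter.
; BeginPlay spawns text actors showing its A/E combo keys, in an arc for Instant combos or a ring for Control and Loop.
; ToggleActivation requires the player inside ActivationTrigger and grows PowerTrigger from zero at bounds-normalized speed, optionally blocking toggles until full size.
; Tick calls Enter/ExitPowerArea as active state and overlap change, deactivating after ActivationDuration at full size.
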(event OnComponentBeginOverlap(PowerTrigger)
  (params (OverlappedComponent :type Primitive%20Component%20Object%20Reference) (OtherActor :type Actor%20Object%20Reference) (OtherComp :type Primitive%20Component%20Object%20Reference) (OtherBodyIndex :type Integer) (bFromSweep :type Boolean) (SweepResult :type Hit%20Result%20Structure%20%28by%20ref%29))
  (Utilities|Casting|CastToGlobalCharacter OtherActor)
  (Variables|Default|SetPlayerInPowerArea true))

(event OnComponentEndOverlap(PowerTrigger)
  (params (OverlappedComponent :type Primitive%20Component%20Object%20Reference) (OtherActor :type Actor%20Object%20Reference) (OtherComp :type Primitive%20Component%20Object%20Reference) (OtherBodyIndex :type Integer))
  (Utilities|Casting|CastToGlobalCharacter OtherActor)
  (Variables|Default|SetPlayerInPowerArea false))

(event OnComponentBeginOverlap(ActivationTrigger)
  (params (OverlappedComponent :type Primitive%20Component%20Object%20Reference) (OtherActor :type Actor%20Object%20Reference) (OtherComp :type Primitive%20Component%20Object%20Reference) (OtherBodyIndex :type Integer) (bFromSweep :type Boolean) (SweepResult :type Hit%20Result%20Structure%20%28by%20ref%29))
  (bind _asglobal_character (Utilities|Casting|CastToGlobalCharacter OtherActor))
  (Variables|/Game/Blueprints/Character/GlobalCharacter.GlobalCharacter_C|SetComboKeys _asglobal_character (Variables|Default|GetComboKeys))
  (Variables|Default|SetPlayerInActivationArea true))

(event OnComponentEndOverlap(ActivationTrigger)
  (params (OverlappedComponent :type Primitive%20Component%20Object%20Reference) (OtherActor :type Actor%20Object%20Reference) (OtherComp :type Primitive%20Component%20Object%20Reference) (OtherBodyIndex :type Integer))
  (Utilities|Casting|CastToGlobalCharacter OtherActor)
  (Variables|Default|SetPlayerInActivationArea false))

(event EventBeginPlay
  (bind _powertrigger (Variables|Default|GetPowerTrigger))
  (bind _combokeys (Variables|Default|GetComboKeys))
  (bind _combokeys_2 (Variables|Default|GetComboKeys))
  (bind _returnvalue (Utilities|Array|Length _combokeys))
  (bind (_min _max) (Components|StaticMesh|GetLocalBounds _powertrigger))
  (bind _returnvalue_2 (/ 120 _returnvalue))
  (bind _returnvalue_3 (* _min -1.0))
  (bind _returnvalue_4 (+ _returnvalue_3 _max))
  (bind _returnvalue_5 (/ _returnvalue_4 2.0))
  (bind _returnvalue_6 (/ "100.000000,100.000000,100.000000" _returnvalue_5))
  (bind (_x _y _z) (Math|Vector|BreakVector _returnvalue_6))
  (Rendering|SetVisibility (Variables|Default|GetPowerTrigger) false false)
  (Variables|Default|SetDefaultScale (Variables|/Script/Engine.SceneComponent|GetRelativeScale3D (Variables|Default|GetPowerTrigger)))
  (Variables|Default|SetExpansionCoefficient (Math|Vector|MakeVector _x (/ (* _y (.y (* (Variables|Default|GetDefaultScale) _returnvalue_4))) (.x (* (Variables|Default|GetDefaultScale) _returnvalue_4))) (/ (* _z (.z (* (Variables|Default|GetDefaultScale) _returnvalue_4))) (.x (* (Variables|Default|GetDefaultScale) _returnvalue_4)))))
  (switch Utilities|FlowControl|Switch|SwitchonPowerCombos (Variables|Default|GetPowerCombo)
    (:NewEnumerator1
      (for (_array_element _array_index) _combokeys
        (bind _returnvalue_7 (Game|SpawnActorfromClass "/Script/Engine.TextRenderActor" (Math|Transform|MakeTransform (+ (* (Math|Vector|GetForwardVector (Math|Rotator|MakeRotator 0.0 0.0 (+ (.yaw (Transformation|GetWorldRotation (Variables|Default|GetStele))) (Math|Conversions|ToFloat(Integer) (+ (* _array_index _returnvalue_2 -1) _returnvalue_2))))) (Math|Float|MakeLiteralFloat 7e+01)) (Transformation|GetWorldLocation (Variables|Default|GetStele)) "0,0,5.000000") (Math|Rotator|MakeRotator (.Roll (Math|Rotator|BreakRotator (Math|Rotator|MakeRotator 0.0 0.0 (+ (.yaw (Transformation|GetWorldRotation (Variables|Default|GetStele))) (Math|Conversions|ToFloat(Integer) (+ (* _array_index _returnvalue_2 -1) _returnvalue_2)))))) 9e+01 (.Yaw (Math|Rotator|BreakRotator (Math|Rotator|MakeRotator 0.0 0.0 (+ (.yaw (Transformation|GetWorldRotation (Variables|Default|GetStele))) (Math|Conversions|ToFloat(Integer) (+ (* _array_index _returnvalue_2 -1) _returnvalue_2)))))))) "Undefined" 0 0))
        (Rendering|Components|TextRender|SetTextRenderColor (Variables|/Script/Engine.TextRenderActor|GetTextRender _returnvalue_7) (Math|Color|MakeColor 0 0 0 0))
        (Rendering|Components|TextRender|SetHorizontalAlignment (Variables|/Script/Engine.TextRenderActor|GetTextRender _returnvalue_7) "EHTA_Center")
        (Class|TextRenderComponent|SetVerticalAlignment (Variables|/Script/Engine.TextRenderActor|GetTextRender _returnvalue_7) "EVRTA_TextCenter")
        (if (== _array_element "A")
          (Rendering|Components|TextRender|SetText (Variables|/Script/Engine.TextRenderActor|GetTextRender _returnvalue_7) (Utilities|Text|MakeLiteralText "A"))
          (elif (== _array_element "E")
            (Rendering|Components|TextRender|SetText (Variables|/Script/Engine.TextRenderActor|GetTextRender _returnvalue_7) (Utilities|Text|MakeLiteralText "E"))))))
    (:NewEnumerator2
      (for (_array_element_2 _array_index_2) _combokeys_2 :!label _label
        (bind _returnvalue_8 (Game|SpawnActorfromClass "/Script/Engine.TextRenderActor" (Math|Transform|MakeTransform (+ (* (Math|Vector|GetForwardVector (Math|Rotator|MakeRotator 0.0 0.0 (+ (.yaw (Transformation|GetWorldRotation (Variables|Default|GetStele))) (Math|Conversions|ToFloat(Integer) (* _array_index_2 (/ 360 (Utilities|Array|Length _combokeys_2)) -1))))) (Math|Float|MakeLiteralFloat 7e+01)) (Transformation|GetWorldLocation (Variables|Default|GetStele)) "0,0,5.000000") (Math|Rotator|MakeRotator (.Roll (Math|Rotator|BreakRotator (Math|Rotator|MakeRotator 0.0 0.0 (+ (.yaw (Transformation|GetWorldRotation (Variables|Default|GetStele))) (Math|Conversions|ToFloat(Integer) (* _array_index_2 (/ 360 (Utilities|Array|Length _combokeys_2)) -1)))))) 9e+01 (.Yaw (Math|Rotator|BreakRotator (Math|Rotator|MakeRotator 0.0 0.0 (+ (.yaw (Transformation|GetWorldRotation (Variables|Default|GetStele))) (Math|Conversions|ToFloat(Integer) (* _array_index_2 (/ 360 (Utilities|Array|Length _combokeys_2)) -1)))))))) "Undefined" 0 0))
        (Rendering|Components|TextRender|SetTextRenderColor (Variables|/Script/Engine.TextRenderActor|GetTextRender _returnvalue_8) (Math|Color|MakeColor 0 0 0 0))
        (Rendering|Components|TextRender|SetHorizontalAlignment (Variables|/Script/Engine.TextRenderActor|GetTextRender _returnvalue_8) "EHTA_Center")
        (Class|TextRenderComponent|SetVerticalAlignment (Variables|/Script/Engine.TextRenderActor|GetTextRender _returnvalue_8) "EVRTA_TextCenter")
        (if (== _array_element_2 "A")
          (Rendering|Components|TextRender|SetText (Variables|/Script/Engine.TextRenderActor|GetTextRender _returnvalue_8) (Utilities|Text|MakeLiteralText "A"))
          (elif (== _array_element_2 "E")
            (Rendering|Components|TextRender|SetText (Variables|/Script/Engine.TextRenderActor|GetTextRender _returnvalue_8) (Utilities|Text|MakeLiteralText "E"))))))
    (:NewEnumerator0
      (goto _label))))

(event EventTick
  (params (DeltaSeconds :type Float%20%28single-precision%29))
  (bind _returnvalue (Game|GetPlayerCharacter 0))
  (bind _asglobal_character (Utilities|Casting|CastToGlobalCharacter _returnvalue))
  (if (Variables|Default|GetIsActive)
    (CallFunction|PowerAreaExpansion DeltaSeconds)
    (if (Math|Vector|Equal(Vector) (Variables|Default|GetDefaultScale) (Variables|/Script/Engine.SceneComponent|GetRelativeScale3D (Variables|Default|GetPowerTrigger)) 0.0001)
      (CallFunction|MakeActivationDuration DeltaSeconds)))
  (if (Math|Boolean|ANDBoolean (Variables|Default|GetIsActive) (Variables|Default|GetPlayerInPowerArea) (not (Variables|Default|GetHasPower)))
    (Default|EnterPowerArea _asglobal_character (Variables|Default|GetareaType))
    (Variables|/Game/Blueprints/Character/GlobalCharacter.GlobalCharacter_C|SetComboKeys _asglobal_character (Variables|Default|GetComboKeys))
    (Variables|Default|SetHasPower true)
    (elif (and (or (not (Variables|Default|GetIsActive)) (not (Variables|Default|GetPlayerInPowerArea))) (Variables|Default|GetHasPower))
      (Default|ExitPowerArea (.AsGlobal%20Character (Utilities|Casting|CastToGlobalCharacter (Game|GetPlayerCharacter 0))) (Variables|Default|GetareaType))
      (Variables|Default|SetHasPower false))))

(fn ConstructionScript)

(fn ToggleActivation
  (bind _powertrigger (Variables|Default|GetPowerTrigger))
  (if (not (Variables|Default|GetWaitPropagationEndToDeactivate))
    (if (Variables|Default|GetPlayerInActivationArea)
      (bind _output_get (Variables|Default|SetIsActive (not (Variables|Default|GetIsActive)) :!label _label))
      (if _output_get
        (Transformation|SetRelativeScale3D _powertrigger "0, 0, 0")
        (Rendering|SetVisibility _powertrigger true false)
        (Variables|Default|SetActualActivationDuration 0.0)
        (else
          (Rendering|SetVisibility _powertrigger false false))))
    (elif (and (Variables|Default|GetPlayerInActivationArea) (Math|Vector|Equal(Vector) (Variables|Default|GetDefaultScale) (Variables|/Script/Engine.SceneComponent|GetRelativeScale3D (Variables|Default|GetPowerTrigger)) 0.0001))
      (goto _label))))

(fn PowerAreaExpansion
  (params (deltatime :type Float%20%28single-precision%29))
  (bind _defaultscale (Variables|Default|GetDefaultScale))
  (bind _powertrigger (Variables|Default|GetPowerTrigger))
  (bind _relativescale3d (Variables|/Script/Engine.SceneComponent|GetRelativeScale3D _powertrigger))
  (if (Math|Boolean|ORBoolean (< (.x _relativescale3d) (.x _defaultscale)) (< (.y _relativescale3d) (.y _defaultscale)) (< (.z _relativescale3d) (.z _defaultscale)))
    (Transformation|SetRelativeScale3D (Variables|Default|GetPowerTrigger) (+ (Variables|/Script/Engine.SceneComponent|GetRelativeScale3D (Variables|Default|GetPowerTrigger)) (* (* (Variables|Default|GetExpansionCoefficient) deltatime) (Variables|Default|GetAreaPropagationSpeed))))
    (else
      (Transformation|SetRelativeScale3D (Variables|Default|GetPowerTrigger) (Variables|Default|GetDefaultScale)))))

(fn MakeActivationDuration
  (params (deltaTime :type Float%20%28single-precision%29))
  (bind _output_get (Variables|Default|SetActualActivationDuration (+ (Variables|Default|GetActualActivationDuration) deltaTime)))
  (if (>= _output_get (Variables|Default|GetActivationDuration))
    (bind _output_get_2 (Variables|Default|SetIsActive false))
    (if (not _output_get_2)
      (Rendering|SetVisibility (Variables|Default|GetPowerTrigger) false false))))