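; Projectile actor for a thrown spear, simulating flight manually in Tick after Shoot supplies the launch velocity and a SpearPhysics acceleration.
; Each tick line-traces the next step on Visibility, ignoring the player pawn, then sweeps forward, faces along Velocity and adds SpearPhysics without delta-time scaling.
; A trace hit stops the spear at its current location, short of the impact point, and enables its collision.
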(event EventTick
  (params (DeltaSeconds :type Float%20%28single-precision%29))
  (bind _returnvalue (Transformation|GetActorLocation))
  (if (Variables|Default|GetisThrowed)
    (bind _output_get (Variables|Default|SetStartTrace (Transformation|GetActorLocation)))
    (Variables|Default|SetEndTrace (+ _output_get (* (Variables|Default|GetVelocity) DeltaSeconds)))
    (bind _returnvalue_2 (Collision|LineTraceByChannel (Variables|Default|GetStartTrace) (Variables|Default|GetEndTrace) "TraceTypeQuery1" false (Utilities|Array|MakeArray (Game|Player|GetPlayerPawn 0)) "ForDuration"))
    (if _returnvalue_2
      (Variables|Default|SetisThrowed false)
      (Variables|Default|SetVelocity "0, 0, 0")
      (Collision|SetActorEnableCollision true)
      (else
        (Transformation|SetActorLocation (Variables|Default|GetEndTrace) true false)
        (Transformation|SetActorRotation (Math|Rotator|FindLookatRotation _returnvalue (+ _returnvalue (Variables|Default|GetVelocity))))
        (Variables|Default|SetVelocity (+ (Variables|Default|GetVelocity) (Variables|Default|GetSpearPhysics)))))))

(fn ConstructionScript)

(fn Shoot
  (params (ShootPower :type Vector) (SpearPhysics :type Vector))
  (Variables|Default|SetisThrowed true)
  (Variables|Default|SetVelocity ShootPower)
  (Variables|Default|SetSpearPhysics SpearPhysics))