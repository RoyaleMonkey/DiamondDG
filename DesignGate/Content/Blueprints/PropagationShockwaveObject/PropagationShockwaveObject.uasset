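; A shockwave relay object that rings a bell and emits an expanding wave when another wave triggers it.
; Tick scales SpreadShockWave up until it reaches twice SpreadRange, then resets it.
; Mesh overlaps start the wave either from the player's Shockwave, if ActivableByShockWave, or otherwise from another relay object.
; On a relay hand-off it stops the sender's wave and sets itself as that sender's PropagationObject, preventing immediate back-propagation.
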(event OnComponentBeginOverlap(StaticMesh)
  (params (OverlappedComponent :type Primitive%20Component%20Object%20Reference) (OtherActor :type Actor%20Object%20Reference) (OtherComp :type Primitive%20Component%20Object%20Reference) (OtherBodyIndex :type Integer) (bFromSweep :type Boolean) (SweepResult :type Hit%20Result%20Structure%20%28by%20ref%29))
  (if (Variables|Default|GetactivableByShockWave)
    (bind _asglobal_character (Utilities|Casting|CastToGlobalCharacter (Game|Player|GetPlayerPawn 0)))
    (if (== (Variables|/Game/Blueprints/Character/GlobalCharacter.GlobalCharacter_C|GetShockwave _asglobal_character) OtherComp)
      (if (not (Variables|Default|GetIsSpreading))
        (Variables|Default|SetIsSpreading true)
        (Audio|SpawnSoundatLocation "/Game/Sounds/Sounds/bell.bell" (Transformation|GetActorLocation) "0, 0, 0" 0.1 (Math|Random|RandomFloatinRange 0.9 1.1) 0.0 0 0 :!label _label)))
    (else
      (bind _aspropagation_shockwave_object (Utilities|Casting|CastToPropagationShockwaveObject OtherActor))
      (if (and (not (Variables|Default|GetIsSpreading)) (!= _aspropagation_shockwave_object (Variables|Default|GetPropagationObject)))
        (Variables|PropagationShockwaveObject_C|SetPropagationObject _aspropagation_shockwave_object self)
        (Transformation|SetWorldScale3D (Variables|PropagationShockwaveObject_C|GetSpreadShockWave _aspropagation_shockwave_object) "0.200000,0.200000,0.200000")
        (Variables|PropagationShockwaveObject_C|SetIsSpreading _aspropagation_shockwave_object false)
        (Variables|Default|SetIsSpreading true)
        (goto _label)))))

(event EventTick
  (params (DeltaSeconds :type Float%20%28single-precision%29))
  (bind _spreadspeed (Variables|Default|GetSpreadSpeed))
  (bind _spreadshockwave (Variables|Default|GetSpreadShockWave))
  (bind _returnvalue (* DeltaSeconds _spreadspeed))
  (if (Variables|Default|GetIsSpreading)
    (Transformation|SetWorldScale3D _spreadshockwave (+ (Math|Vector|MakeVector _returnvalue _returnvalue _returnvalue) (Transformation|GetWorldScale _spreadshockwave)))
    (if (>= (.x (Transformation|GetWorldScale (Variables|Default|GetSpreadShockWave))) (* (Variables|Default|GetSpreadRange) 2.0))
      (Transformation|SetWorldScale3D (Variables|Default|GetSpreadShockWave) "0.200000,0.200000,0.200000")
      (Variables|Default|SetIsSpreading false))))

(fn ConstructionScript)