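; Squall actor that pushes physics-simulating objects that begin overlapping it.
; On BeginPlay it copies SquallPower from the player's GlobalCharacter.
; On overlap it applies an impulse to static mesh roots along the direction away from itself, scaled by that power.
; The squall's world location is added to the impulse's X and Y, and its own height alone serves as Z.
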(event EventBeginPlay
  ;[1 1 1] Get Squall Power from character
  (bind _asglobal_character (Utilities|Casting|CastToGlobalCharacter (Game|GetPlayerCharacter 0)))
  (Variables|Default|SetsquallPower (Variables|/Game/Blueprints/Character/GlobalCharacter.GlobalCharacter_C|GetsquallPower _asglobal_character)))

(event Collision|EventActorBeginOverlap
  (params (OtherActor :type Actor%20Object%20Reference))
  (bind _returnvalue (Transformation|GetActorLocation))
  (bind _rootcomponent (Variables|/Script/Engine.Actor|GetRootComponent OtherActor))
  ;[1 1 1] Push physical objects
  (if (Physics|IsSimulatingPhysics _rootcomponent "None")
    (bind _asstatic_mesh_component (Utilities|Casting|CastToStaticMeshComponent _rootcomponent))
    (Physics|AddImpulse _asstatic_mesh_component (Math|Vector|MakeVector (.x (+ (* (Math|Vector|GetUnitDirection(Vector) (Transformation|GetActorLocation) (Transformation|GetWorldLocation _asstatic_mesh_component)) (* 1e+03 (Variables|Default|GetsquallPower))) _returnvalue)) (.y (+ (* (Math|Vector|GetUnitDirection(Vector) (Transformation|GetActorLocation) (Transformation|GetWorldLocation _asstatic_mesh_component)) (* 1e+03 (Variables|Default|GetsquallPower))) _returnvalue)) (.Z (Math|Vector|BreakVector _returnvalue))) "None" false)))

(fn ConstructionScript)