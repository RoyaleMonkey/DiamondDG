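; Test actor, likely a projectile for checking sphere shield collision going by its name, that flies in a straight line along negative world X.
; Tick moves it at constant speed with a swept location update and accumulates elapsed time, destroying it once the lifetime is reached.
; Any actor overlap also destroys it immediately, while the Hit event is empty and a debug print is left disconnected.
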(event EventTick
  (params (DeltaSeconds :type Float%20%28single-precision%29))
  (Transformation|SetActorLocation (+ (Transformation|GetActorLocation) (* (Math|Vector|MakeVector -1e+03 0.0 0.0) DeltaSeconds)) true false)
  (bind _output_get (Variables|Default|SetActualLifeTime (+ (Variables|Default|GetActualLifeTime) DeltaSeconds)))
  (if (>= _output_get (Variables|Default|GetLifeTime))
    (Actor|DestroyActor)))

(event Collision|EventActorBeginOverlap
  (params (OtherActor :type Actor%20Object%20Reference))
  (Actor|DestroyActor))

(event Collision|EventHit
  (params (MyComp :type Primitive%20Component%20Object%20Reference) (Other :type Actor%20Object%20Reference) (OtherComp :type Primitive%20Component%20Object%20Reference) (bSelfMoved :type Boolean) (HitLocation :type Vector :default "0, 0, 0") (HitNormal :type Vector :default "0, 0, 0") (NormalImpulse :type Vector :default "0, 0, 0") (Hit :type Hit%20Result%20Structure%20%28by%20ref%29)))

(fn ConstructionScript)