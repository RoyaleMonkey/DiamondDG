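; Test teleporter actor that moves the player character to a level or spot chosen by its Destination enum.
; On BeginPlay, it labels its TextRender with the destination name and sets the Plane's material.
; When a GlobalCharacter overlaps it, HUB, Art and Features open levels by name.
; Sandbox does nothing on overlap; the other destinations move the character to the ArrivalPoint's world location via SetActorRelativeLocation.
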(event EventBeginPlay
  (bind _textrender (Variables|Default|GetTextRender))
  (bind _plane (Variables|Default|GetPlane))
  (switch Utilities|FlowControl|Switch|SwitchonTeleportDestEnum (Variables|Default|GetDestination)
    (:NewEnumerator0
      (Rendering|Components|TextRender|SetText _textrender (Utilities|Text|MakeLiteralText "HUB"))
      (Rendering|Material|SetMaterial _plane 0 0))
    (:NewEnumerator1
      (Rendering|Components|TextRender|SetText _textrender (Utilities|Text|MakeLiteralText "Art Scene"))
      (Rendering|Material|SetMaterial _plane 0 0))
    (:NewEnumerator2
      (Rendering|Components|TextRender|SetText _textrender (Utilities|Text|MakeLiteralText "Features Scene"))
      (Rendering|Material|SetMaterial _plane 0 0 :!label _label))
    (:NewEnumerator3
      (Rendering|Components|TextRender|SetText _textrender (Utilities|Text|MakeLiteralText "Sandbox"))
      (Rendering|Material|SetMaterial _plane 0 0))
    (:NewEnumerator4
      (Rendering|Components|TextRender|SetText _textrender (Utilities|Text|MakeLiteralText "GliderTower"))
      (goto _label))
    (:NewEnumerator5
      (Rendering|Components|TextRender|SetText _textrender (Utilities|Text|MakeLiteralText "Geyser"))
      (Rendering|Material|SetMaterial _plane 0 0))
    (:NewEnumerator6
      (Rendering|Components|TextRender|SetText _textrender (Utilities|Text|MakeLiteralText "Dash"))
      (Rendering|Material|SetMaterial _plane 0 0))
    (:NewEnumerator7
      (Rendering|Components|TextRender|SetText _textrender (Utilities|Text|MakeLiteralText "Squall"))
      (Rendering|Material|SetMaterial _plane 0 0))
    (:NewEnumerator8
      (Rendering|Components|TextRender|SetText _textrender (Utilities|Text|MakeLiteralText "Shockwave"))
      (Rendering|Material|SetMaterial _plane 0 0))))

(event Collision|EventActorBeginOverlap
  (params (OtherActor :type Actor%20Object%20Reference))
  (bind _asglobal_character (Utilities|Casting|CastToGlobalCharacter OtherActor))
  (switch Utilities|FlowControl|Switch|SwitchonTeleportDestEnum (Variables|Default|GetDestination)
    (:NewEnumerator0
      (Game|OpenLevel(byName) "HubScene"))
    (:NewEnumerator1
      (Game|OpenLevel(byName) "Yoan"))
    (:NewEnumerator2
      (Game|OpenLevel(byName) "GlobalTestScene"))
    (:NewEnumerator4
      (Transformation|SetActorRelativeLocation _asglobal_character (Transformation|GetWorldLocation (Variables|Default|GetarrivalPoint)) :!label _label))
    (:NewEnumerator5
      (goto _label))
    (:NewEnumerator6
      (goto _label))
    (:NewEnumerator7
      (goto _label))
    (:NewEnumerator8
      (goto _label))))

(event EventTick
  (params (DeltaSeconds :type Float%20%28single-precision%29)))

(fn ConstructionScript)