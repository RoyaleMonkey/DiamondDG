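; Lance projectile actor that flies in an arc once thrown.
; Shoot sets the thrown flag and scales the given direction into a launch velocity.
; While thrown, Tick line-traces along each step, ignoring the player pawn, then moves and orients the lance along its velocity as a per-frame downward pull bends it.
; A trace hit zeroes velocity and stops it short of the impact point.
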(event EventTick
  (params (DeltaSeconds :type Float%20%28single-precision%29))
  (bind _returnvalue (Transformation|GetActorLocation))
  (if (Variables|Default|GetisThrowed)
    (bind _output_get (Variables|Default|SetStartTrace (Transformation|GetActorLocation)))
    (Variables|Default|SetEndTrace (+ _output_get (* (Variables|Default|GetVelocity) DeltaSeconds)))
    (bind _returnvalue_2 (Collision|LineTraceByChannel (Variables|Default|GetStartTrace) (Variables|Default|GetEndTrace) "TraceTypeQuery1" false (Utilities|Array|MakeArray (Game|Player|GetPlayerPawn 0)) "ForDuration"))
    (if _returnvalue_2
      (Variables|Default|SetisThrowed false)
      (Variables|Default|SetVelocity "0, 0, 0")
      (else
        (Transformation|SetActorLocation (Variables|Default|GetEndTrace) false false)
        (Transformation|SetActorRotation (Math|Rotator|FindLookatRotation _returnvalue (+ _returnvalue (Variables|Default|GetVelocity))))
        (Variables|Default|SetVelocity (+ (Variables|Default|GetVelocity) "0.000000, 0,-20.000000"))))))

(fn ConstructionScript)

(fn Shoot
  (params (ShootDirection :type Vector))
  (Variables|Default|SetisThrowed true)
  (Variables|Default|SetVelocity (* ShootDirection 2e+03)))